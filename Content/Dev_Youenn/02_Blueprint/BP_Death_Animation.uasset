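; BP_Death_Animation is a placed actor that stages the death animation scene.
; On BeginPlay it registers itself with Louis's player controller and hides its spotlight.
; Move_Camera lights the spotlight, teleports the first BP_Camera_Louis to a target point and resets the world camera's field of view.
; A separate Trigger_Montage event plays the death montage on its killer skeletal mesh.
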(event Custom|Move_Camera
  ;[0.15 0.15 0.15 0.5] Positionne la caméra pour l'animation de mort
  (Rendering|SetVisibility (Variables|Default|GetSpot_Light) true false)
  (bind _outactors (Actor|GetAllActorsOfClass "/Game/Dev_Louis/02_Blueprint/01_Game_Management/Rooms/BP_Camera_Louis.BP_Camera_Louis_C"))
  (Transformation|SetWorldTransform (Variables|/Script/Engine.Actor|GetRootComponent (Utilities|Array|Get(acopy) _outactors)) (Transformation|GetActorTransform (Variables|Default|GetTargetPoint)) false true)
  (Camera|SetFieldOfView (Variables|/Game/Dev_Louis/02_Blueprint/01_Game_Management/Rooms/BP_Camera_Louis.BP_Camera_Louis_C|GetCamera (Variables|/Game/Dev_Louis/02_Blueprint/03_Player/BP_ThirdPersonPlayerController_Louis.BP_ThirdPersonPlayerController_Louis_C|GetWorld_Camera (CallFunction|GetPlayerControllerLouis))) 9e+01))

(event Custom|Trigger_Montage
  ;[0.15 0.15 0.15 0.5] Lancer l'animation de mort
  (Animation|Montage|PlayMontage (Variables|Default|GetA_Killer_IdleA) (Variables|Default|GetDeath_Animation_Montagre) 1.0 0.0 "None" false))

(event EventBeginPlay
  (Variables|/Game/Dev_Louis/02_Blueprint/03_Player/BP_ThirdPersonPlayerController_Louis.BP_ThirdPersonPlayerController_Louis_C|SetDeath_Animation (CallFunction|GetPlayerControllerLouis) self)
  (Rendering|SetVisibility (Variables|Default|GetSpot_Light) false false))

(fn ConstructionScript)