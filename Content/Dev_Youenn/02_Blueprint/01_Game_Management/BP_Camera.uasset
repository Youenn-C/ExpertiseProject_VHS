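; BP_Camera is a placeable camera actor that takes over player 0's view when the player character enters its trigger box.
; On BeginPlay, the instance flagged IsFirst becomes the initial view target, and every instance applies its own FOV to its camera component.
; Box overlap switches the view target to this actor with no blend time set, and nothing runs on Tick.
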(event OnComponentBeginOverlap(Box)
  (params (OverlappedComponent :type Primitive%20Component%20Object%20Reference) (OtherActor :type Actor%20Object%20Reference) (OtherComp :type Primitive%20Component%20Object%20Reference) (OtherBodyIndex :type Integer) (bFromSweep :type Boolean) (SweepResult :type Hit%20Result%20Structure%20%28by%20ref%29))
  (if (== OtherActor (CallFunction|GetPlayerCharacterYouenn))
    (Game|Player|SetViewTargetwithBlend (Game|GetPlayerController 0) self 0.0 "VTBlend_Linear" 0.0 false)))

(event EventBeginPlay
  (if (Variables|Default|GetisFirst)
    (Game|Player|SetViewTargetwithBlend (Game|GetPlayerController 0) self 0.0 "VTBlend_Linear" 0.0 false))
  (Camera|SetFieldOfView (Variables|Default|GetCamera) (Variables|Default|GetFOV)))

(event EventTick
  (params (DeltaSeconds :type Float%20%28single-precision%29)))

(fn ConstructionScript)