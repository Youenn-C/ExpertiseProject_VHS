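; BP_Checkpoint is a checkpoint that sets the player's respawn point and triggers a save of player data.
; The checkpoint flagged IsFirst registers itself on BeginPlay, and any checkpoint registers itself with the player controller when the player character overlaps its box collider.
; Overlap also saves through the VHS game instance unless the player is dying.
; A Debug variable mirrors the saved data for tracking only.
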(event OnComponentBeginOverlap(Box_Collider)
  (params (OverlappedComponent :type Primitive%20Component%20Object%20Reference) (OtherActor :type Actor%20Object%20Reference) (OtherComp :type Primitive%20Component%20Object%20Reference) (OtherBodyIndex :type Integer) (bFromSweep :type Boolean) (SweepResult :type Hit%20Result%20Structure%20%28by%20ref%29))
  (if (== OtherActor (CallFunction|GetPlayerCharacterYouenn))
    (Variables|/Game/Dev_Youenn/02_Blueprint/03_Player/BP_Player_Controller_Youenn.BP_Player_Controller_Youenn_C|SetRespawn_Point (CallFunction|GetPlayerControllerYouenn) self)
    (if (not (Variables|/Game/Dev_Youenn/02_Blueprint/03_Player/BP_Player_Controller_Youenn.BP_Player_Controller_Youenn_C|GetIs_Dying (CallFunction|GetPlayerControllerYouenn)))
      (CallFunction|SaveDatafromPlayer))))

(event Custom|Save_Data_From_Player
  (bind _perma_inventory (Default|SaveDatafromPlayer (CallFunction|GetVHSInstance)))
  (Variables|Default|SetDebug _perma_inventory))

(event EventBeginPlay
  (if (Variables|Default|GetIs_First)
    (Variables|/Game/Dev_Youenn/02_Blueprint/03_Player/BP_Player_Controller_Youenn.BP_Player_Controller_Youenn_C|SetRespawn_Point (CallFunction|GetPlayerControllerYouenn) self))
  ;[0.15 0.15 0.15 0.5] Ne sert qu'a suivra l'évolution de la sauvegarde
  (Variables|Default|SetDebug (Variables|/Game/Dev_Youenn/02_Blueprint/01_Game_Management/BP_VHS_Instance.BP_VHS_Instance_C|GetPerma_Inventory (CallFunction|GetVHSInstance))))

(fn ConstructionScript)