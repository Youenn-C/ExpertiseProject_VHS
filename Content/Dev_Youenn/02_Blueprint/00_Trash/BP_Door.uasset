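; BP_Door is a clickable door actor that swings open when approached, with debug prints on its events.
; Clicking either side's mouse detector runs Activate, which passes the door's location to the player controller's CallCharacterMovement.
; Overlapping the side A player detector calls the door opening, where a timeline interpolates the Door component's yaw from closed to open position.
; Side B has no overlap handler, and no closing logic is present.
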(event OnComponentBeginOverlap(PlayerDetectorSideA)
  (params (OverlappedComponent :type Primitive%20Component%20Object%20Reference) (OtherActor :type Actor%20Object%20Reference) (OtherComp :type Primitive%20Component%20Object%20Reference) (OtherBodyIndex :type Integer) (bFromSweep :type Boolean) (SweepResult :type Hit%20Result%20Structure%20%28by%20ref%29))
  (Development|PrintString "Hello")
  (CallFunction|OpenDoor))

(event OnClicked(MouseDetectorSideA)
  (params (TouchedComponent :type Primitive%20Component%20Object%20Reference) (ButtonPressed :type Key%20Structure :default "None"))
  (CallFunction|Activate)
  (Development|PrintString "clic On Side A !"))

(event OnClicked(MouseDetectorSideB)
  (params (TouchedComponent :type Primitive%20Component%20Object%20Reference) (ButtonPressed :type Key%20Structure :default "None"))
  (CallFunction|Activate)
  (Development|PrintString "clic On Side B !"))

(event Custom|Open_Door
  (Development|PrintString "Hello there")
  (Components|Timeline|SetPlayRate (Variables|Default|GetT_Openin_Door) 1.0)
  (bind _anim (Timeline|T_Openin_Door PlayFromStart)
    (:Update
      (Transformation|SetRelativeRotation (Variables|Default|GetDoor) (Math|Rotator|MakeRotator 0.0 0.0 (Math|Float|Lerp (Variables|Default|GetClose_Position) (Variables|Default|GetOpen_Position) _anim)) false false))))

(event EventActivate
  (bind _returnvalue (Transformation|GetActorLocation))
  (Default|CallCharacterMovement (CallFunction|GetPlayerControllerYouenn) 1e+01 _returnvalue _returnvalue))

(fn ConstructionScript)