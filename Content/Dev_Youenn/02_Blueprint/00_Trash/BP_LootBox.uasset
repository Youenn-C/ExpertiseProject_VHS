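; BP_LootBox is a clickable actor that moves the ThirdPersonCharacterYouenn character to a target point, with no loot logic yet.
; BeginPlay enables mouse-over and click events on player controller 0, and the MouseDetector component prints French debug messages on hover and click.
; A click calls Activate, which uses MoveComponentTo on the character's capsule, passing the TargetPoint sprite's world location as the relative target.
; An unconnected character-movement node is left unused.
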(event OnBeginCursorOver(MouseDetector)
  (params (TouchedComponent :type Primitive%20Component%20Object%20Reference))
  (Development|PrintString "La sourie est là"))

(event OnEndCursorOver(MouseDetector)
  (params (TouchedComponent :type Primitive%20Component%20Object%20Reference))
  (Development|PrintString "La sourie n'est plus là"))

(event OnClicked(MouseDetector)
  (params (TouchedComponent :type Primitive%20Component%20Object%20Reference) (ButtonPressed :type Key%20Structure :default "None"))
  (CallFunction|Activate)
  (Development|PrintString "clic !"))

(event Custom|Activate
  (Components|MoveComponentTo (Variables|/Script/Engine.Character|GetCapsuleComponent (CallFunction|GetThirdPersonCharacterYouenn)) (Transformation|GetWorldLocation (Variables|/Script/Engine.TargetPoint|GetSpriteComponent (Variables|Default|GetTarget_Point))) "0, 0, 0" false false 0.2 false))

(event EventBeginPlay
  (bind _returnvalue (Game|GetPlayerController 0))
  (Variables|/Script/Engine.PlayerController|SetbEnableMouseOverEvents _returnvalue true)
  (Variables|/Script/Engine.PlayerController|SetbEnableClickEvents _returnvalue true))

(fn ConstructionScript)