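; Touch-driven player controller that creates the player UI, forwards target-movement requests to the player character and handles death.
; Vertical swipes run timelines that slide a map overlay and toggle whether world interaction is allowed, while touch presses trace and print the object under the finger.
; Death, also triggered by releasing H, waits, reopens the main level and reloads savables.
; The VHS instance supplies the saved lever state and permanent inventory.
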(event Custom|LoadSave
  (bind _value (Default|GetSavedValue (CallFunction|GetVHSInstance) "/Game/Dev_Youenn/02_Blueprint/02_Gameplay_Elements/BP_IO_SO_Lever.BP_IO_SO_Lever_C"))
  (Variables|//---INVENTORY---\\|SetHave_Lever (> _value 0)))

(event Custom|Call_Target_Movement
  (params (World%20Location :type Vector) (Permission :type Float%20%28double-precision%29))
  ;[0.15 0.15 0.15 0.5] Character Movement
  (Default|TargetMovement (Variables|Default|GetPlayer_Character_Youenn) World%20Location Permission))

(event Custom|Death
  ;[0.15 0.15 0.15 0.5] Death and Respawn
  (Variables|//---BOOL---\\|SetIs_Dying true)
  (Development|PrintString "JE MEURE !!!!")
  (Utilities|FlowControl|Delay 3.0)
  (CallFunction|Respawn))

(event Custom|Respawn
  ;[0.15 0.15 0.15 0.5] Death and Respawn
  (Game|OpenLevel(byName) "Lvl_Main_Youenn")
  (CallFunction|ReloadSavable)
  ;;[0.15 0.15 0.15 0.5] Permet de ne pas trigger la save de datas
  (Utilities|FlowControl|Delay 1.0)
  (Variables|//---BOOL---\\|SetIs_Dying false))

(event EventBeginPlay
  (bind _returnvalue (Game|GetPlayerController 0))
  ;[0.15 0.15 0.15 0.5] Initialisation
  (if (Pawn|IsLocalPlayerController)
    (Utilities|FlowControl|Sequence
      (:then_0
        (bind _asbp_player_character_youenn (Utilities|Casting|CastToBP_Player_Character_Youenn (Pawn|GetControlledPawn)))
        (Variables|Default|SetPlayer_Character_Youenn _asbp_player_character_youenn))
      (:then_1
        (Variables|Default|SetbShowMouseCursor true)
        (Variables|/Script/Engine.PlayerController|SetbEnableMouseOverEvents _returnvalue true)
        (Variables|/Script/Engine.PlayerController|SetbEnableClickEvents _returnvalue true))
      (:then_2
        (bind _returnvalue_2 (UserInterface|CreateWidget "/Game/Dev_Youenn/02_Blueprint/03_Player/WBP_Player_UI_Youenn.WBP_Player_UI_Youenn_C" self))
        (Variables|/Game/Dev_Youenn/02_Blueprint/03_Player/WBP_Player_UI_Youenn.WBP_Player_UI_Youenn_C|SetNewVar _returnvalue_2 self)
        (bind _output_get (Variables|Default|SetPlayer_UI _returnvalue_2))
        (UserInterface|Viewport|AddtoViewport _output_get 0))
      (:then_3
        (Variables|//---INVENTORY---\\|SetTempProgression (Variables|/Game/Dev_Youenn/02_Blueprint/01_Game_Management/BP_VHS_Instance.BP_VHS_Instance_C|GetPerma_Inventory (CallFunction|GetVHSInstance)))))))

(event Input|KeyboardEvents|H
  (params (Key :type Key%20Structure :default "None"))
  ;[0.15 0.15 0.15 0.5] Death and Respawn
  (:Released
    (CallFunction|Death)))

(event Input|TouchEvents|InputTouch
  (params (Location :type Vector) (FingerIndex :type ETouchIndex%20Enum))
  (bind (_bblockinghit _hitactor _hitcomponent) (CallFunction|GetClickedGameObject))
  (bind _returnvalue (Math|Vector2D|MakeVector2D (.x Location) (.y Location)))
  ;[0.15 0.15 0.15 0.5] Mobile Inputs
  (:Pressed
    (Variables|//---MAP---\\|SetTouch_Start_Pos _returnvalue)
    (Variables|//---BOOL---\\|SetTouching true)
    ;;[0.15 0.15 0.15 0.5] Get Clicked GameObject
    (if _bblockinghit
      (Development|PrintString (Utilities|GetDisplayName _hitactor))
      (Development|PrintString (Utilities|GetDisplayName _hitcomponent))))
  (:Released
    (bind _output_get (Variables|//---MAP---\\|SetTouch_Start_Pos ""))
    (Variables|//---MAP---\\|SetTouch_End_Pos _output_get))
  (:Moved
    (Variables|//---MAP---\\|SetTouch_End_Pos _returnvalue)
    (if (Variables|//---BOOL---\\|GetTouching)
      ;;[0.15 0.15 0.15 0.5] Open and Close Map by slide
      (if (not (Variables|//---MAP---\\|GetMap_Is_Moving))
        (Utilities|FlowControl|Sequence
          (:then_0
            (if (> (.y (- (Variables|//---MAP---\\|GetTouch_Start_Pos) (Variables|//---MAP---\\|GetTouch_End_Pos))) (Variables|Default|GetTouch_Move_Amount))
              (if (not (Variables|//---MAP---\\|GetMap_Is_Close))
                (Variables|//---MAP---\\|SetMap_Is_Moving true)
                (Variables|//---MAP---\\|SetAllow_To_Interact_Whis_World true)
                (Development|PrintString "UP")
                (Components|Timeline|SetPlayRate (Variables|Default|GetT_Map_Close) (Variables|//---MAP---\\|GetMap_Play_Rate))
                (bind _open_map (Timeline|T_Map_Close PlayFromStart)
                  (:Update
                    (Class|Widget|SetRenderTransform (Variables|/Game/Dev_Youenn/02_Blueprint/03_Player/WBP_Player_UI_Youenn.WBP_Player_UI_Youenn_C|GetOverlay_54 (Variables|Default|GetPlayer_UI)) (Utilities|Struct|MakeWidgetTransform (Math|Vector2D|MakeVector2D 0.0 (Math|Float|Lerp (Variables|//---MAP---\\|GetMap_Close_Y_Pos) (Variables|//---MAP---\\|GetMap_Open_Y_Pos) _open_map)) "(X=1.000000,Y=1.000000)" "(X=0.000000,Y=0.000000)" 0.0)))
                  (:Finished
                    (Variables|//---MAP---\\|SetMap_Is_Moving false)
                    (Variables|//---MAP---\\|SetMap_Is_Close true))))))
          (:then_1
            (if (< (.y (- (Variables|//---MAP---\\|GetTouch_Start_Pos) (Variables|//---MAP---\\|GetTouch_End_Pos))) (* (Variables|Default|GetTouch_Move_Amount) -1.0))
              (if (Variables|//---MAP---\\|GetMap_Is_Close)
                (Variables|//---MAP---\\|SetMap_Is_Moving true)
                (Variables|//---MAP---\\|SetAllow_To_Interact_Whis_World false)
                (Development|PrintString "DOWN")
                (Components|Timeline|SetPlayRate (Variables|Default|GetT_Map_Open) (Variables|//---MAP---\\|GetMap_Play_Rate))
                (bind _open_map_2 (Timeline|T_Map_Open PlayFromStart)
                  (:Update
                    (Class|Widget|SetRenderTransform (Variables|/Game/Dev_Youenn/02_Blueprint/03_Player/WBP_Player_UI_Youenn.WBP_Player_UI_Youenn_C|GetOverlay_54 (Variables|Default|GetPlayer_UI)) (Utilities|Struct|MakeWidgetTransform (Math|Vector2D|MakeVector2D 0.0 (Math|Float|Lerp (Variables|//---MAP---\\|GetMap_Close_Y_Pos) (Variables|//---MAP---\\|GetMap_Open_Y_Pos) _open_map_2)) "(X=1.000000,Y=1.000000)" "(X=0.000000,Y=0.000000)" 0.0)))
                  (:Finished
                    (Variables|//---MAP---\\|SetMap_Is_Moving false)
                    (Variables|//---MAP---\\|SetMap_Is_Close false)))))))))))

(fn ConstructionScript)

(fn GetClickedGameObject
  (bind _hitresult (Class|PlayerController|GetHitResultUnderFingerbyChannel "Touch1" "TraceTypeQuery3" true))
  (bind (_bblockinghit _binitialoverlap _time _distance _location _impactpoint _normal _impactnormal _physmat _hitactor _hitcomponent) (Collision|BreakHitResult _hitresult))
  (return _bblockinghit _hitactor _hitcomponent))