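; Player character Blueprint for point-to-move navigation on the navmesh.
; On BeginPlay it registers itself with the Youenn player controller and switches movement to NavWalking.
; Character_Movement line-traces the Visibility channel along a supplied world ray and uses SimpleMoveToLocation toward the hit, offset along X by the Permision input.
; Target_Movement skips the trace and moves directly to a given world location.
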(event Custom|Character_Movement
  (params (World_Location :type Vector) (World_Direction :type Vector) (Permision :type Float%20%28double-precision%29))
  (bind (_outhit _returnvalue) (Collision|LineTraceByChannel World_Location (+ World_Location (* World_Direction 1e+04)) "TraceTypeQuery1" false 0 "None"))
  (if _returnvalue
    (AI|Navigation|SimpleMovetoLocation (CallFunction|GetPlayerControllerYouenn) (Math|Vector|MakeVector (- (.X (Math|Vector|BreakVector (.Location (Collision|BreakHitResult _outhit)))) Permision) (.Y (Math|Vector|BreakVector (.Location (Collision|BreakHitResult _outhit)))) (.Z (Math|Vector|BreakVector (.Location (Collision|BreakHitResult _outhit))))))))

(event Custom|Target_Movement
  (params (World%20Location :type Vector))
  (AI|Navigation|SimpleMovetoLocation (CallFunction|GetPlayerControllerYouenn) World%20Location))

(event EventBeginPlay
  (Variables|/Game/Dev_Youenn/02_Blueprint/03_Player/BP_Player_Controller_Youenn.BP_Player_Controller_Youenn_C|SetPlayer_Character_Youenn (CallFunction|GetPlayerControllerYouenn) self)
  (Pawn|Components|CharacterMovement|SetMovementMode (Variables|Character|GetCharacterMovement) "MOVE_NavWalking" 0))

(fn ConstructionScript)