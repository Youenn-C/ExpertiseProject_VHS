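; Touch-driven lever interactive object that the player must own, install in place, then switch on once.
; A touch checks world-interaction permission and lever possession, then installs or activates it if in range, otherwise requests player movement toward it.
; Installing shows the mesh and activating rotates it to the ON position.
; Progress saves as an integer (empty, installed, activated) through TempSave, and AfterLoad replays the matching step.
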(event OnInputTouchBegin(Collider)
  (params (FingerIndex :type ETouchIndex%20Enum :default "Touch1") (TouchedComponent :type Primitive%20Component%20Object%20Reference))
  (if (not (Variables|Default|GetAs%20Interact))
    (if (Variables|/Game/Dev_Youenn/02_Blueprint/03_Player/BP_Player_Controller_Youenn.BP_Player_Controller_Youenn_C|GetAllow_To_Interact_Whis_World (CallFunction|GetPlayerControllerYouenn))
      (Variables|Default|SetAs%20Interact true)
      (CallFunction|Activate))))

(event Custom|Activate_Lever
  (Variables|Default|SetAs%20Interact false)
  (Variables|Default|SetAs_Been_Activated true)
  (Transformation|SetRelativeRotation (Variables|Default|GetLever) (Variables|Default|GetPosition_ON) false false)
  (CallFunction|PreSave))

(event Custom|Install_Lever
  (Rendering|SetVisibility (Variables|Default|GetLever) true true)
  (Variables|Default|SetLever_is_Install true)
  (Variables|Default|SetAs%20Interact false)
  (CallFunction|PreSave))

(event EventActivate
  (if (Variables|/Game/Dev_Youenn/02_Blueprint/03_Player/BP_Player_Controller_Youenn.BP_Player_Controller_Youenn_C|GetHave_Lever (CallFunction|GetPlayerControllerYouenn))
    (if (Variables|Default|GetLever_is_Install)
      (if (Variables|Default|GetPlayer_Is_In_Range)
        (if (not (Variables|Default|GetAs_Been_Activated))
          (CallFunction|ActivateLever)
          (Development|PrintString "Levier activer"))
        (else
          (Development|PrintString "Mouvement" :!label _label)
          (Default|CallTargetMovement (CallFunction|GetPlayerControllerYouenn) (Transformation|GetActorLocation) 2e+01)))
      (elif (Variables|Default|GetPlayer_Is_In_Range)
        (CallFunction|InstallLever)
        (Development|PrintString "levier placer")
        (else
          (goto _label))))
    (else
      (Development|PrintString "Levier non possèdé"))))

(event EventPreSave
  (Variables|Default|SetObject_Value (+ (Math|Integer|SelectInt 1 0 (Variables|Default|GetAs_Been_Activated)) (Math|Integer|SelectInt 1 0 (Variables|Default|GetLever_is_Install))))
  (CallFunction|TempSave))

(event EventAfterLoad
  (params (Int_Value :type Integer))
  (if (> Int_Value 0)
    (if (> Int_Value 1)
      (bind _output_get (Variables|Default|SetLever_is_Install true))
      (Variables|Default|SetAs_Been_Activated _output_get)
      (CallFunction|ActivateLever)
      (else
        (Variables|Default|SetLever_is_Install true)
        (Variables|Default|SetAs_Been_Activated false)
        (CallFunction|InstallLever)))
    (else
      (Rendering|SetVisibility (Variables|Default|GetLever) false false))))

(fn ConstructionScript)