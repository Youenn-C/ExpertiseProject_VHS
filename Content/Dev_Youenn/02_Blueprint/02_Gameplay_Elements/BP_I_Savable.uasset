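; Base Blueprint for savable gameplay elements that store and restore a single Value, keyed by the object's class.
; TempSave adds Value to the player controller's TempProgression map, and LoadSavable reads it back from the VHS instance before calling AfterLoad.
; AfterLoad and PreSave are empty hook events, and PreSave is not called within this Blueprint.
; Class keying means instances of the same class share one saved entry.
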(event Custom|LoadSavable
  (bind _value (Default|GetSavedValue (CallFunction|GetVHSInstance) (Utilities|GetClass self)))
  (Variables|Default|SetValue _value)
  (CallFunction|AfterLoad))

(event Custom|AfterLoad)

(event Custom|PreSave)

(event Custom|TempSave
  (Utilities|Map|Add (Variables|/Game/Dev_Youenn/02_Blueprint/03_Player/BP_Player_Controller_Youenn.BP_Player_Controller_Youenn_C|GetTempProgression (CallFunction|GetPlayerControllerYouenn)) (Utilities|GetClass self) (Variables|Default|GetValue)))

(fn ConstructionScript
  (|CallParentFunction))