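; Base Blueprint for savable objects that persist a single ObjectValue keyed by the object's class, so instances of the same class share one saved entry.
; Half a second after BeginPlay it reads the saved value from the VHS instance and passes it to the empty AfterLoad hook.
; TempSave writes the current value into the player controller's TempProgression map, and PreSave is another empty hook.
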(event Custom|LoadSavable
  (bind _value (Default|GetSavedValue (CallFunction|GetVHSInstance) (Utilities|GetClass self)))
  (bind _output_get (Variables|SaveDatas|SetObject_Value _value))
  (CallFunction|AfterLoad _output_get))

(event Custom|AfterLoad
  (params (Int_Value :type Integer)))

(event Custom|PreSave)

(event Custom|TempSave
  (Utilities|Map|Add (Variables|/Game/Dev_Louis/02_Blueprint/03_Player/BP_ThirdPersonPlayerController_Louis.BP_ThirdPersonPlayerController_Louis_C|GetTempProgression (CallFunction|GetPlayerControllerLouis)) (Utilities|GetClass self) (Variables|SaveDatas|GetObject_Value)))

(event EventBeginPlay
  (Utilities|FlowControl|Delay 0.5)
  (CallFunction|LoadSavable))

(fn ConstructionScript
  (|CallParentFunction))