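; Interactable object Blueprint that tracks whether the player character is within range of it.
; Overlap events on its Player_Detector component set and clear PlayerIsInRange, ignoring any actor other than the player character.
; When the player enters while AsInteract is true, it calls Activate, an event left empty here that serves as a hook for the actual interaction.
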(event OnComponentEndOverlap(Player_Detector)
  (params (OverlappedComponent :type Primitive%20Component%20Object%20Reference) (OtherActor :type Actor%20Object%20Reference) (OtherComp :type Primitive%20Component%20Object%20Reference) (OtherBodyIndex :type Integer))
  (if (== OtherActor (CallFunction|GetPlayerCharacterYouenn))
    (Variables|Default|SetPlayer_Is_In_Range false)))

(event OnComponentBeginOverlap(Player_Detector)
  (params (OverlappedComponent :type Primitive%20Component%20Object%20Reference) (OtherActor :type Actor%20Object%20Reference) (OtherComp :type Primitive%20Component%20Object%20Reference) (OtherBodyIndex :type Integer) (bFromSweep :type Boolean) (SweepResult :type Hit%20Result%20Structure%20%28by%20ref%29))
  (if (== OtherActor (CallFunction|GetPlayerCharacterYouenn))
    (Variables|Default|SetPlayer_Is_In_Range true)
    (if (Variables|Default|GetAs%20Interact)
      (CallFunction|Activate))))

(event Custom|Activate)

(fn ConstructionScript)