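; BP_IO_VideoRecorder is a touch-driven interactable object that ends in the victory screen when the player holds the enchanted hammer.
; A touch on its collider checks the player controller's interaction and hammer flags, latches HaveInteract, locks interaction, then calls Activate.
; In range, Activate spawns a fountain particle effect, disables world interaction and displays WBP_Victory_Screen.
; Out of range, it calls TriggerMovement instead.
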(event OnInputTouchBegin(Collider)
  (params (FingerIndex :type ETouchIndex%20Enum :default "Touch1") (TouchedComponent :type Primitive%20Component%20Object%20Reference))
  (if (Variables|/Game/Dev_Youenn/02_Blueprint/03_Player/BP_Player_Controller_Youenn.BP_Player_Controller_Youenn_C|GetAllow%20Interaction (CallFunction|GetPlayerControllerYouenn))
    (if (not (Variables|Default|GetHave_Interact))
      (if (Variables|/Game/Dev_Youenn/02_Blueprint/03_Player/BP_Player_Controller_Youenn.BP_Player_Controller_Youenn_C|GetAllow_To_Interact_Whis_World (CallFunction|GetPlayerControllerYouenn))
        (if (Variables|/Game/Dev_Youenn/02_Blueprint/03_Player/BP_Player_Controller_Youenn.BP_Player_Controller_Youenn_C|GetHave_Enchant_Hammer (CallFunction|GetPlayerControllerYouenn))
          (Variables|Default|SetHave_Interact true)
          (Variables|/Game/Dev_Youenn/02_Blueprint/03_Player/BP_Player_Controller_Youenn.BP_Player_Controller_Youenn_C|SetAllow%20Interaction (CallFunction|GetPlayerControllerYouenn) false)
          (CallFunction|Activate))))))

(event EventActivate
  (bind _asbp_player_controller_youenn (CallFunction|GetPlayerControllerYouenn))
  (if (Variables|/Game/Dev_Youenn/02_Blueprint/03_Player/BP_Player_Controller_Youenn.BP_Player_Controller_Youenn_C|GetHave_Enchant_Hammer (CallFunction|GetPlayerControllerYouenn))
    (if (Variables|Default|GetPlayer_Is_In_Range)
      (Niagara|SpawnSystematLocation "/Niagara/DefaultAssets/Templates/Systems/FountainLightweight.FountainLightweight" (Transformation|GetActorLocation))
      (bind _output_get (Variables|/Game/Dev_Youenn/02_Blueprint/03_Player/BP_Player_Controller_Youenn.BP_Player_Controller_Youenn_C|SetAllow%20Interaction _asbp_player_controller_youenn false))
      (Variables|/Game/Dev_Youenn/02_Blueprint/03_Player/BP_Player_Controller_Youenn.BP_Player_Controller_Youenn_C|SetAllow_To_Interact_Whis_World _asbp_player_controller_youenn _output_get)
      (bind _returnvalue (UserInterface|CreateWidget "/Game/Dev_Youenn/02_Blueprint/03_Player/WBP_Victory_Screen.WBP_Victory_Screen_C" (CallFunction|GetPlayerControllerYouenn)))
      (UserInterface|Viewport|AddtoViewport _returnvalue 0)
      (else
        (CallFunction|TriggerMovement)))))

(fn ConstructionScript
  (|CallParentFunction))