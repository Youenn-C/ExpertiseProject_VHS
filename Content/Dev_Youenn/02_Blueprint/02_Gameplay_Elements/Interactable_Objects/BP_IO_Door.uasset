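; Touch-operated interactable door that the player character passes through from either side.
; A touch records the side and locks interaction on the player controller, then opens the door if the player is in range or sends them to that side's entry point.
; Opening is a timeline yaw rotation that then sends the player to the opposite exit point.
; After a timeline-length delay, a second timeline closes the door and restores interaction.
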(event OnInputTouchBegin(TouchDetectorSideB)
  (params (FingerIndex :type ETouchIndex%20Enum :default "Touch1") (TouchedComponent :type Primitive%20Component%20Object%20Reference))
  ;[0.15 0.15 0.15 0.5] Récupération de l'information du clic
  (if (Variables|/Game/Dev_Youenn/02_Blueprint/03_Player/BP_Player_Controller_Youenn.BP_Player_Controller_Youenn_C|GetAllow%20Interaction (CallFunction|GetPlayerControllerYouenn))
    (if (not (Variables|Default|GetHave_Interact))
      (if (Variables|/Game/Dev_Youenn/02_Blueprint/03_Player/BP_Player_Controller_Youenn.BP_Player_Controller_Youenn_C|GetAllow_To_Interact_Whis_World (CallFunction|GetPlayerControllerYouenn))
        (Variables|Default|SetHave_Interact true)
        (Variables|/Game/Dev_Youenn/02_Blueprint/03_Player/BP_Player_Controller_Youenn.BP_Player_Controller_Youenn_C|SetAllow%20Interaction (CallFunction|GetPlayerControllerYouenn) false)
        (CallFunction|Activate)))))

(event OnInputTouchBegin(TouchDetectorSideA)
  (params (FingerIndex :type ETouchIndex%20Enum :default "Touch1") (TouchedComponent :type Primitive%20Component%20Object%20Reference))
  ;[0.15 0.15 0.15 0.5] Récupération de l'information du clic
  (if (Variables|/Game/Dev_Youenn/02_Blueprint/03_Player/BP_Player_Controller_Youenn.BP_Player_Controller_Youenn_C|GetAllow%20Interaction (CallFunction|GetPlayerControllerYouenn))
    (Variables|//--BOOLEAN--\\|SetAs_Clic_On_Side_A true)
    (if (not (Variables|Default|GetHave_Interact))
      (if (Variables|/Game/Dev_Youenn/02_Blueprint/03_Player/BP_Player_Controller_Youenn.BP_Player_Controller_Youenn_C|GetAllow_To_Interact_Whis_World (CallFunction|GetPlayerControllerYouenn))
        (Variables|Default|SetHave_Interact true)
        (Variables|/Game/Dev_Youenn/02_Blueprint/03_Player/BP_Player_Controller_Youenn.BP_Player_Controller_Youenn_C|SetAllow%20Interaction (CallFunction|GetPlayerControllerYouenn) false)
        (CallFunction|Activate)))))

(event Custom|Open_Door
  (bind _t_open_door (Variables|Default|GetT_Open_Door))
  ;[0.15 0.15 0.15 0.5] Ouverture de la porte
  (if (Variables|//--BOOLEAN--\\|GetAllow_Movement)
    (Components|Timeline|SetPlayRate _t_open_door 1.0)
    (Variables|//--FLOAT--\\|SetDelay (Components|Timeline|GetTimelineLength _t_open_door))
    (bind _deltatime (Timeline|T_Open_Door PlayFromStart)
      (:Update
        (Transformation|SetActorRelativeRotation (Math|Rotator|MakeRotator 0.0 0.0 (Math|Float|Lerp (Variables|//--FLOAT--\\|GetClose_Position) (Variables|//--FLOAT--\\|GetOpen_Position) _deltatime))))
      (:Finished
        (Variables|Default|SetHave_Interact false)
        (if (Variables|//--BOOLEAN--\\|GetAs_Clic_On_Side_A)
          (Default|CallTargetMovement (CallFunction|GetPlayerControllerYouenn) (Transformation|GetActorLocation (Variables|//--TARGETPOINT--\\|GetTargetPoint_Out_B)) 0.0)
          (else
            (Default|CallTargetMovement (CallFunction|GetPlayerControllerYouenn) (Transformation|GetActorLocation (Variables|//--TARGETPOINT--\\|GetTargetPoint_Out_A)) 0.0)))
        (Utilities|FlowControl|Delay (Variables|//--FLOAT--\\|GetDelay))
        (Components|Timeline|SetPlayRate (Variables|Default|GetT_Open_Door) 1.0)
        (bind _deltatime_2 (Timeline|T_Close_Door PlayFromStart)
          (:Update
            (Transformation|SetActorRelativeRotation (Math|Rotator|MakeRotator 0.0 0.0 (Math|Float|Lerp (Variables|//--FLOAT--\\|GetClose_Position) (Variables|//--FLOAT--\\|GetOpen_Position) _deltatime_2))))
          (:Finished
            (bind _output_get (Variables|//--BOOLEAN--\\|SetAllow_Movement false))
            (Variables|//--BOOLEAN--\\|SetAs_Clic_On_Side_A _output_get)
            (Variables|/Game/Dev_Youenn/02_Blueprint/03_Player/BP_Player_Controller_Youenn.BP_Player_Controller_Youenn_C|SetAllow%20Interaction (CallFunction|GetPlayerControllerYouenn) true)))))))

(event EventActivate
  ;[0.15 0.15 0.15 0.5] Activation
  (if (Variables|Default|GetHave_Interact)
    (if (Variables|Default|GetPlayer_Is_In_Range)
      (Variables|//--BOOLEAN--\\|SetAllow_Movement true)
      (CallFunction|OpenDoor)
      (elif (Variables|//--BOOLEAN--\\|GetAs_Clic_On_Side_A)
        ;;[0.15 0.15 0.15 0.5] Si cliqué sur la face A
        (Default|CallTargetMovement (CallFunction|GetPlayerControllerYouenn) (Transformation|GetActorLocation (Variables|//--TARGETPOINT--\\|GetTargetPoint_In_A)) 0.0)
        (else
          ;;[0.15 0.15 0.15 0.5] Si cliqué sur la face B
          (Default|CallTargetMovement (CallFunction|GetPlayerControllerYouenn) (Transformation|GetActorLocation (Variables|//--TARGETPOINT--\\|GetTargetPoint_In_B)) 0.0))))))

(fn ConstructionScript)