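; Interactable enchantment table that lets a player carrying the hammer enchant it once by touching the table.
; Touch input checks the player controller's interaction flags, then Activate either calls TriggerMovement when the player is out of range or performs the enchantment.
; Enchanting sets the controller's enchanted-hammer flag, briefly shows a hammer mesh and spawns an effect at the table between delays.
; The hammer's PreSave runs after either branch.
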(event OnInputTouchBegin(Collider)
  (params (FingerIndex :type ETouchIndex%20Enum :default "Touch1") (TouchedComponent :type Primitive%20Component%20Object%20Reference))
  (if (Variables|/Game/Dev_Louis/02_Blueprint/03_Player/BP_ThirdPersonPlayerController_Louis.BP_ThirdPersonPlayerController_Louis_C|GetAllowInteraction (CallFunction|GetPlayerControllerLouis))
    (if (not (Variables|Default|GetHas%20Interact))
      (if (Variables|/Game/Dev_Louis/02_Blueprint/03_Player/BP_ThirdPersonPlayerController_Louis.BP_ThirdPersonPlayerController_Louis_C|GetAllowInteractionWithWorld (CallFunction|GetPlayerControllerLouis))
        (Variables|Default|SetHas%20Interact true)
        (CallFunction|Activate)))))

(event EventBeginPlay
  (Rendering|SetVisibility (Variables|Default|GetHammer_Part_01) false true))

(event EventActivate
  (if (Variables|/Game/Dev_Louis/02_Blueprint/03_Player/BP_ThirdPersonPlayerController_Louis.BP_ThirdPersonPlayerController_Louis_C|GetHaveHammer (CallFunction|GetPlayerControllerLouis))
    (if (Variables|Default|GetHas%20Interact)
      (if (Variables|/Game/Dev_Louis/02_Blueprint/03_Player/BP_ThirdPersonPlayerController_Louis.BP_ThirdPersonPlayerController_Louis_C|GetHaveEnchantHammer (CallFunction|GetPlayerControllerLouis))
        (Variables|Default|SetHas%20Interact false)
        (else
          (if (Variables|Default|GetPlayer_Is_In_Range)
            (Variables|/Game/Dev_Louis/02_Blueprint/03_Player/BP_ThirdPersonPlayerController_Louis.BP_ThirdPersonPlayerController_Louis_C|SetHaveEnchantHammer (CallFunction|GetPlayerControllerLouis) true)
            (Rendering|SetVisibility (Variables|Default|GetHammer_Part_01) true true)
            (Utilities|FlowControl|Delay 1.0)
            (Niagara|SpawnSystematLocation 0 (Transformation|GetWorldLocation (Variables|Default|GetTable_Part_02)))
            (Utilities|FlowControl|Delay 1.0)
            (Rendering|SetVisibility (Variables|Default|GetHammer_Part_01) false true)
            (Variables|Default|SetHas%20Interact false)
            (Development|PrintString "Vous enchantez le marteau")
            (else
              (CallFunction|TriggerMovement)))
          (Default|PreSave (Variables|Default|GetHammer)))))
    (else
      (Variables|Default|SetHas%20Interact false))))

(fn ConstructionScript
  (|CallParentFunction))