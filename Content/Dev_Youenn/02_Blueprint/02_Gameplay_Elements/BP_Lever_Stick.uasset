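; Touch-interactable lever stick pickup that grants the player a lever.
; A touch, when world interaction is allowed, either collects it in range or calls the player controller to move toward it, retrying on detector overlap.
; Collection sets HaveLever; the progression write and hiding occur only if the map lookup for a "None" key succeeds.
; Reset only makes the stick visible again.
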(event OnInputTouchBegin(Collider)
  (params (FingerIndex :type ETouchIndex%20Enum :default "Touch1") (TouchedComponent :type Primitive%20Component%20Object%20Reference))
  (if (not (Variables|Default|GetAs_Interact))
    (if (Variables|/Game/Dev_Youenn/02_Blueprint/03_Player/BP_Player_Controller_Youenn.BP_Player_Controller_Youenn_C|GetAllow_To_Interact_Whis_World (CallFunction|GetPlayerControllerYouenn))
      (Variables|Default|SetAs_Interact true)
      (CallFunction|Activate))))

(event OnComponentBeginOverlap(Player_Detector)
  (params (OverlappedComponent :type Primitive%20Component%20Object%20Reference) (OtherActor :type Actor%20Object%20Reference) (OtherComp :type Primitive%20Component%20Object%20Reference) (OtherBodyIndex :type Integer) (bFromSweep :type Boolean) (SweepResult :type Hit%20Result%20Structure%20%28by%20ref%29))
  (if (== OtherActor (CallFunction|GetPlayerCharacterYouenn))
    (Variables|Default|SetPlayer_Is_In_Range true)
    (if (Variables|Default|GetAs_Interact)
      (CallFunction|Activate))))

(event OnComponentEndOverlap(Player_Detector)
  (params (OverlappedComponent :type Primitive%20Component%20Object%20Reference) (OtherActor :type Actor%20Object%20Reference) (OtherComp :type Primitive%20Component%20Object%20Reference) (OtherBodyIndex :type Integer))
  (if (== OtherActor (CallFunction|GetPlayerCharacterYouenn))
    (Variables|Default|SetPlayer_Is_In_Range false)))

(event EventReset
  (Rendering|SetVisibility (Variables|Default|GetDefaultSceneRoot) true true))

(event EventActivate
  (if (Variables|Default|GetAs_Interact)
    (if (Variables|Default|GetPlayer_Is_In_Range)
      (Variables|/Game/Dev_Youenn/02_Blueprint/03_Player/BP_Player_Controller_Youenn.BP_Player_Controller_Youenn_C|SetHave_Lever (CallFunction|GetPlayerControllerYouenn) true)
      (if (.ReturnValue (Utilities|Map|Find (Variables|/Game/Dev_Youenn/02_Blueprint/03_Player/BP_Player_Controller_Youenn.BP_Player_Controller_Youenn_C|GetPlayer_Progression (CallFunction|GetPlayerControllerYouenn)) ""))
        (Utilities|Map|Add (Variables|/Game/Dev_Youenn/02_Blueprint/03_Player/BP_Player_Controller_Youenn.BP_Player_Controller_Youenn_C|GetPlayer_Progression (CallFunction|GetPlayerControllerYouenn)) "" true)
        (Rendering|SetVisibility (Variables|Default|GetDefaultSceneRoot) false true)
        (Variables|Default|SetAs_Interact false))
      (else
        (Default|CallTargetMovement (CallFunction|GetPlayerControllerYouenn) (Transformation|GetActorLocation) 2e+01)))))

(fn ConstructionScript
  (|CallParentFunction))