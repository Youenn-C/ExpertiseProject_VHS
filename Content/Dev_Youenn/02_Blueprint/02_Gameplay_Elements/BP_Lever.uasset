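; Touch-driven lever mount actor: the player installs a carried lever, hidden at start, then can activate it.
; Touching the collider, when the player controller allows interaction, runs Activate, which requires HaveLever and checks the detector's player-range flag.
; Out of range, it requests player movement toward the actor and clears the interaction flag; in range, it places or activates the lever.
; Activation itself only prints debug text and resets that flag.
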(event OnInputTouchBegin(Collider)
  (params (FingerIndex :type ETouchIndex%20Enum :default "Touch1") (TouchedComponent :type Primitive%20Component%20Object%20Reference))
  (if (not (Variables|Default|GetAs_Interact))
    (if (Variables|/Game/Dev_Youenn/02_Blueprint/03_Player/BP_Player_Controller_Youenn.BP_Player_Controller_Youenn_C|GetAllow_To_Interact_Whis_World (CallFunction|GetPlayerControllerYouenn))
      (Variables|Default|SetAs_Interact true)
      (CallFunction|Activate))))

(event OnComponentBeginOverlap(Player_Detector)
  (params (OverlappedComponent :type Primitive%20Component%20Object%20Reference) (OtherActor :type Actor%20Object%20Reference) (OtherComp :type Primitive%20Component%20Object%20Reference) (OtherBodyIndex :type Integer) (bFromSweep :type Boolean) (SweepResult :type Hit%20Result%20Structure%20%28by%20ref%29))
  (if (== OtherActor (CallFunction|GetPlayerCharacterYouenn))
    (Variables|Default|SetPlayer_Is_In_Range true)
    (if (Variables|Default|GetAs_Interact)
      (CallFunction|Activate))))

(event OnComponentEndOverlap(Player_Detector)
  (params (OverlappedComponent :type Primitive%20Component%20Object%20Reference) (OtherActor :type Actor%20Object%20Reference) (OtherComp :type Primitive%20Component%20Object%20Reference) (OtherBodyIndex :type Integer))
  (if (== OtherActor (CallFunction|GetPlayerCharacterYouenn))
    (Variables|Default|SetPlayer_Is_In_Range false)))

(event Custom|Activate_Lever
  (Development|PrintString "Hello")
  (Variables|Default|SetAs_Interact false))

(event Custom|Unplace_Lever
  (Rendering|SetVisibility (Variables|Default|GetLever) false true))

(event Custom|Place_Lever
  (Rendering|SetVisibility (Variables|Default|GetLever) true true)
  (Variables|Default|SetLever_is_Install true))

(event EventBeginPlay
  (Rendering|SetVisibility (Variables|Default|GetLever) false false))

(event EventActivate
  (if (Variables|/Game/Dev_Youenn/02_Blueprint/03_Player/BP_Player_Controller_Youenn.BP_Player_Controller_Youenn_C|GetHave_Lever (CallFunction|GetPlayerControllerYouenn))
    (if (Variables|Default|GetLever_is_Install)
      (if (Variables|Default|GetPlayer_Is_In_Range)
        (CallFunction|ActivateLever)
        (Development|PrintString "Levier activer")
        (else
          (Development|PrintString "Mouvement" :!label _label)
          (Default|CallTargetMovement (CallFunction|GetPlayerControllerYouenn) (Transformation|GetActorLocation) 2e+01)
          (Variables|Default|SetAs_Interact false)))
      (elif (Variables|Default|GetPlayer_Is_In_Range)
        (CallFunction|PlaceLever)
        (Development|PrintString "levier placer")
        (Variables|Default|SetAs_Interact false)
        (else
          (goto _label))))
    (else
      (Development|PrintString "Levier no possèder")
      (Variables|Default|SetAs_Interact false))))

(fn ConstructionScript)