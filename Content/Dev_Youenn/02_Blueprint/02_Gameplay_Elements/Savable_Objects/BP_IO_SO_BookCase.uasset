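; Savable touch-interactable bookcase whose left and right double doors and four drawers each open once.
; Collider touches flag the chosen part and call Activate, which plays its Timeline if the player is in range, otherwise requests player movement and saves.
; Player interaction locks during opening, then the used collider drops away.
; The saved value is the controller's HaveHammer flag rather than open states; loading restores it and hides the bookcase when true.
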(event OnInputTouchBegin(Left_Up_Drower_Collider)
  (params (FingerIndex :type ETouchIndex%20Enum :default "Touch1") (TouchedComponent :type Primitive%20Component%20Object%20Reference))
  (if (Variables|/Game/Dev_Youenn/02_Blueprint/03_Player/BP_Player_Controller_Youenn.BP_Player_Controller_Youenn_C|GetAllow%20Interaction (CallFunction|GetPlayerControllerYouenn))
    (Variables|//---UPDRAWERS---\\|SetClicked_On_Left_Up_Drower true)
    (if (Rendering|IsVisible (Variables|Default|GetDefaultSceneRoot))
      (if (not (Variables|Default|GetHave_Interact))
        (if (Variables|/Game/Dev_Youenn/02_Blueprint/03_Player/BP_Player_Controller_Youenn.BP_Player_Controller_Youenn_C|GetAllow_To_Interact_Whis_World (CallFunction|GetPlayerControllerYouenn))
          (Variables|Default|SetHave_Interact true)
          (CallFunction|Activate))))))

(event OnInputTouchBegin(Left_Down_Drower_Collider)
  (params (FingerIndex :type ETouchIndex%20Enum :default "Touch1") (TouchedComponent :type Primitive%20Component%20Object%20Reference))
  (if (Variables|/Game/Dev_Youenn/02_Blueprint/03_Player/BP_Player_Controller_Youenn.BP_Player_Controller_Youenn_C|GetAllow%20Interaction (CallFunction|GetPlayerControllerYouenn))
    (Variables|//---DOWNDRAWERS---\\|SetClicked_On_Left_Down_Drower true)
    (if (Rendering|IsVisible (Variables|Default|GetDefaultSceneRoot))
      (if (not (Variables|Default|GetHave_Interact))
        (if (Variables|/Game/Dev_Youenn/02_Blueprint/03_Player/BP_Player_Controller_Youenn.BP_Player_Controller_Youenn_C|GetAllow_To_Interact_Whis_World (CallFunction|GetPlayerControllerYouenn))
          (Variables|Default|SetHave_Interact true)
          (CallFunction|Activate))))))

(event OnInputTouchBegin(Left_Doors_Collider)
  (params (FingerIndex :type ETouchIndex%20Enum :default "Touch1") (TouchedComponent :type Primitive%20Component%20Object%20Reference))
  (if (Variables|/Game/Dev_Youenn/02_Blueprint/03_Player/BP_Player_Controller_Youenn.BP_Player_Controller_Youenn_C|GetAllow%20Interaction (CallFunction|GetPlayerControllerYouenn))
    (Variables|//---LEFTDOORS---\\|SetClicked_On_Left_Doors true)
    (if (Rendering|IsVisible (Variables|Default|GetDefaultSceneRoot))
      (if (not (Variables|Default|GetHave_Interact))
        (if (Variables|/Game/Dev_Youenn/02_Blueprint/03_Player/BP_Player_Controller_Youenn.BP_Player_Controller_Youenn_C|GetAllow_To_Interact_Whis_World (CallFunction|GetPlayerControllerYouenn))
          (Variables|Default|SetHave_Interact true)
          (CallFunction|Activate))))))

(event OnInputTouchBegin(Right_Down_Drower_Collider)
  (params (FingerIndex :type ETouchIndex%20Enum :default "Touch1") (TouchedComponent :type Primitive%20Component%20Object%20Reference))
  (if (Variables|/Game/Dev_Youenn/02_Blueprint/03_Player/BP_Player_Controller_Youenn.BP_Player_Controller_Youenn_C|GetAllow%20Interaction (CallFunction|GetPlayerControllerYouenn))
    (Variables|//---DOWNDRAWERS---\\|SetClicked_On_Right_Down_Drower true)
    (if (Rendering|IsVisible (Variables|Default|GetDefaultSceneRoot))
      (if (not (Variables|Default|GetHave_Interact))
        (if (Variables|/Game/Dev_Youenn/02_Blueprint/03_Player/BP_Player_Controller_Youenn.BP_Player_Controller_Youenn_C|GetAllow_To_Interact_Whis_World (CallFunction|GetPlayerControllerYouenn))
          (Variables|Default|SetHave_Interact true)
          (CallFunction|Activate))))))

(event OnInputTouchBegin(Right_Up_Drower_Collider)
  (params (FingerIndex :type ETouchIndex%20Enum :default "Touch1") (TouchedComponent :type Primitive%20Component%20Object%20Reference))
  (if (Variables|/Game/Dev_Youenn/02_Blueprint/03_Player/BP_Player_Controller_Youenn.BP_Player_Controller_Youenn_C|GetAllow%20Interaction (CallFunction|GetPlayerControllerYouenn))
    (Variables|//---UPDRAWERS---\\|SetClicked_On_Right_Up_Drower true)
    (if (Rendering|IsVisible (Variables|Default|GetDefaultSceneRoot))
      (if (not (Variables|Default|GetHave_Interact))
        (if (Variables|/Game/Dev_Youenn/02_Blueprint/03_Player/BP_Player_Controller_Youenn.BP_Player_Controller_Youenn_C|GetAllow_To_Interact_Whis_World (CallFunction|GetPlayerControllerYouenn))
          (Variables|Default|SetHave_Interact true)
          (CallFunction|Activate))))))

(event OnInputTouchBegin(Right_Doors_Collider)
  (params (FingerIndex :type ETouchIndex%20Enum :default "Touch1") (TouchedComponent :type Primitive%20Component%20Object%20Reference))
  (if (Variables|/Game/Dev_Youenn/02_Blueprint/03_Player/BP_Player_Controller_Youenn.BP_Player_Controller_Youenn_C|GetAllow%20Interaction (CallFunction|GetPlayerControllerYouenn))
    (Variables|//---RIGHTDOORS---\\|SetClicked_On_Right_Doors true)
    (if (Rendering|IsVisible (Variables|Default|GetDefaultSceneRoot))
      (if (not (Variables|Default|GetHave_Interact))
        (if (Variables|/Game/Dev_Youenn/02_Blueprint/03_Player/BP_Player_Controller_Youenn.BP_Player_Controller_Youenn_C|GetAllow_To_Interact_Whis_World (CallFunction|GetPlayerControllerYouenn))
          (Variables|Default|SetHave_Interact true)
          (CallFunction|Activate))))))

(event EventActivate
  (Variables|/Game/Dev_Youenn/02_Blueprint/03_Player/BP_Player_Controller_Youenn.BP_Player_Controller_Youenn_C|SetAllow%20Interaction (CallFunction|GetPlayerControllerYouenn) false)
  (if (Variables|Default|GetHave_Interact)
    (if (Variables|Default|GetPlayer_Is_In_Range)
      (if (Variables|//---RIGHTDOORS---\\|GetClicked_On_Right_Doors)
        (bind _progression (Timeline|T_Right_Doors_Opening PlayFromStart)
          (:Update
            (Transformation|SetRelativeRotation (Variables|Default|GetRight_R_Door) (Math|Rotator|MakeRotator 0.0 0.0 (Math|Float|Lerp (Variables|//---RIGHTDOORS---\\|GetRight_R_Doors_Close_Position) (Variables|//---RIGHTDOORS---\\|GetRight_R_Doors_Open_Position) _progression)) false false)
            (Transformation|SetRelativeRotation (Variables|Default|GetRight_L_Door) (Math|Rotator|MakeRotator 0.0 0.0 (Math|Float|Lerp (Variables|//---RIGHTDOORS---\\|GetRight_L_Doors_Close_Position) (Variables|//---RIGHTDOORS---\\|GetRight_L_Doors_Open_Position) _progression)) false false))
          (:Finished
            (bind _output_get (Variables|//---RIGHTDOORS---\\|SetClicked_On_Right_Doors false))
            (Variables|Default|SetHave_Interact _output_get)
            (Transformation|SetRelativeLocation (Variables|Default|GetRight_Doors_Collider) "0.000000,0.000000,-100.000000" false true)
            (Variables|/Game/Dev_Youenn/02_Blueprint/03_Player/BP_Player_Controller_Youenn.BP_Player_Controller_Youenn_C|SetAllow%20Interaction (CallFunction|GetPlayerControllerYouenn) true)))
        (elif (Variables|//---UPDRAWERS---\\|GetClicked_On_Right_Up_Drower)
          (bind _progression_2 (Timeline|T_Right_Up_Drawer_Opening PlayFromStart)
            (:Update
              (Transformation|SetRelativeLocation (Variables|Default|GetRight_Up_Drawer) (Math|Vector|MakeVector (Math|Float|Lerp (Variables|//---UPDRAWERS---\\|GetUp_Drawers_Close_Position) (Variables|//---UPDRAWERS---\\|GetUp_Drawers_Open_Position) _progression_2) 0.0 0.0) true false))
            (:Finished
              (bind _output_get_2 (Variables|//---UPDRAWERS---\\|SetClicked_On_Right_Up_Drower false))
              (Variables|Default|SetHave_Interact _output_get_2)
              (Transformation|SetRelativeLocation (Variables|Default|GetRight_Up_Drower_Collider) "0.000000,0.000000,-100.000000" false true)
              (Variables|/Game/Dev_Youenn/02_Blueprint/03_Player/BP_Player_Controller_Youenn.BP_Player_Controller_Youenn_C|SetAllow%20Interaction (CallFunction|GetPlayerControllerYouenn) true)))
          (elif (Variables|//---DOWNDRAWERS---\\|GetClicked_On_Right_Down_Drower)
            (bind _progression_3 (Timeline|T_Right_Down_Drawer_Opening PlayFromStart)
              (:Update
                (Transformation|SetRelativeLocation (Variables|Default|GetRight_Down_Drawer) (Math|Vector|MakeVector (Math|Float|Lerp (Variables|//---DOWNDRAWERS---\\|GetDown_Drawers_Close_Position) (Variables|//---DOWNDRAWERS---\\|GetDown_Drawers_Open_Position) _progression_3) 0.0 0.0) true false))
              (:Finished
                (bind _output_get_3 (Variables|//---DOWNDRAWERS---\\|SetClicked_On_Right_Down_Drower false))
                (Variables|Default|SetHave_Interact _output_get_3)
                (Transformation|SetRelativeLocation (Variables|Default|GetRight_Down_Drower_Collider) "0.000000,0.000000,-100.000000" false true)
                (Variables|/Game/Dev_Youenn/02_Blueprint/03_Player/BP_Player_Controller_Youenn.BP_Player_Controller_Youenn_C|SetAllow%20Interaction (CallFunction|GetPlayerControllerYouenn) true)))
            (elif (Variables|//---LEFTDOORS---\\|GetClicked_On_Left_Doors)
              (bind _progression_4 (Timeline|T_Left_Doors_Opening PlayFromStart)
                (:Update
                  (Transformation|SetRelativeRotation (Variables|Default|GetLeft_R_Door) (Math|Rotator|MakeRotator 0.0 0.0 (Math|Float|Lerp (Variables|//---LEFTDOORS---\\|GetLeft_R_Doors_Close_Position) (Variables|//---LEFTDOORS---\\|GetLeft_R_Doors_Open_Position) _progression_4)) false false)
                  (Transformation|SetRelativeRotation (Variables|Default|GetLeft_L_Door) (Math|Rotator|MakeRotator 0.0 0.0 (Math|Float|Lerp (Variables|//---LEFTDOORS---\\|GetLeft_L_Doors_Close_Position) (Variables|//---LEFTDOORS---\\|GetLeft_L_Doors_Open_Position) _progression_4)) false false))
                (:Finished
                  (bind _output_get_4 (Variables|//---LEFTDOORS---\\|SetClicked_On_Left_Doors false))
                  (Variables|Default|SetHave_Interact _output_get_4)
                  (Transformation|SetRelativeLocation (Variables|Default|GetLeft_Doors_Collider) "0.000000,0.000000,-100.000000" false true)
                  (Variables|/Game/Dev_Youenn/02_Blueprint/03_Player/BP_Player_Controller_Youenn.BP_Player_Controller_Youenn_C|SetAllow%20Interaction (CallFunction|GetPlayerControllerYouenn) true)))
              (elif (Variables|//---UPDRAWERS---\\|GetClicked_On_Left_Up_Drower)
                (bind _progression_5 (Timeline|T_Left_Up_Drawer_Opening PlayFromStart)
                  (:Update
                    (Transformation|SetRelativeLocation (Variables|Default|GetLeft_Up_Drawer) (Math|Vector|MakeVector (Math|Float|Lerp (Variables|//---UPDRAWERS---\\|GetUp_Drawers_Close_Position) (Variables|//---UPDRAWERS---\\|GetUp_Drawers_Open_Position) _progression_5) 0.0 0.0) true false))
                  (:Finished
                    (bind _output_get_5 (Variables|//---UPDRAWERS---\\|SetClicked_On_Left_Up_Drower false))
                    (Variables|Default|SetHave_Interact _output_get_5)
                    (Transformation|SetRelativeLocation (Variables|Default|GetLeft_Up_Drower_Collider) "0.000000,0.000000,-100.000000" false true)
                    (Variables|/Game/Dev_Youenn/02_Blueprint/03_Player/BP_Player_Controller_Youenn.BP_Player_Controller_Youenn_C|SetAllow%20Interaction (CallFunction|GetPlayerControllerYouenn) true)))
                (elif (Variables|//---DOWNDRAWERS---\\|GetClicked_On_Left_Down_Drower)
                  (bind _progression_6 (Timeline|T_Left_Down_Drawer_Opening PlayFromStart)
                    (:Update
                      (Transformation|SetRelativeLocation (Variables|Default|GetLeft_Down_Drawer) (Math|Vector|MakeVector (Math|Float|Lerp (Variables|//---DOWNDRAWERS---\\|GetDown_Drawers_Close_Position) (Variables|//---DOWNDRAWERS---\\|GetDown_Drawers_Open_Position) _progression_6) 0.0 0.0) false true))
                    (:Finished
                      (bind _output_get_6 (Variables|//---DOWNDRAWERS---\\|SetClicked_On_Left_Down_Drower false))
                      (Variables|Default|SetHave_Interact _output_get_6)
                      (Transformation|SetRelativeLocation (Variables|Default|GetLeft_Down_Drower_Collider) "0.000000,0.000000,-100.000000" false true)
                      (Variables|/Game/Dev_Youenn/02_Blueprint/03_Player/BP_Player_Controller_Youenn.BP_Player_Controller_Youenn_C|SetAllow%20Interaction (CallFunction|GetPlayerControllerYouenn) true)))
                  (else
                    (CallFunction|PreSave :!label _label))))))))
      (else
        (Default|CallTargetMovement (CallFunction|GetPlayerControllerYouenn) (Transformation|GetActorLocation (Variables|Default|GetPlayer_Position)) (Variables|Default|GetPermission))
        (goto _label)))))

(event EventPreSave
  (Variables|Default|SetObject_Value (Math|Integer|SelectInt 1 0 (Variables|/Game/Dev_Youenn/02_Blueprint/03_Player/BP_Player_Controller_Youenn.BP_Player_Controller_Youenn_C|GetHave_Hammer (CallFunction|GetPlayerControllerYouenn))))
  (CallFunction|TempSave))

(event EventAfterLoad
  (params (Int_Value :type Integer))
  (bind _output_get (Variables|/Game/Dev_Youenn/02_Blueprint/03_Player/BP_Player_Controller_Youenn.BP_Player_Controller_Youenn_C|SetHave_Hammer (CallFunction|GetPlayerControllerYouenn) (Utilities|Select :Index Int_Value :Option%200 false :Option%201 true)))
  (if _output_get
    (Rendering|SetVisibility (Variables|Default|GetDefaultSceneRoot) false true)))

(fn ConstructionScript
  (|CallParentFunction))