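; Savable, touch-interactive dresser whose upper and lower drawers each open once.
; A tap plays the player's interaction montage and opens that drawer if in range, otherwise calls TriggerMovement.
; Timelines slide the drawer, then drop its collider, save, and increment the Enemy's action count.
; Both drawer states pack into one integer, which AfterLoad decodes to replay the openings, rerunning those completion effects.
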(event OnInputTouchEnd(Down_Drower_Collider)
  (params (FingerIndex :type ETouchIndex%20Enum :default "Touch1") (TouchedComponent :type Primitive%20Component%20Object%20Reference))
  (if (Variables|/Game/Dev_Louis/02_Blueprint/03_Player/BP_ThirdPersonPlayerController_Louis.BP_ThirdPersonPlayerController_Louis_C|GetAllowInteraction (CallFunction|GetPlayerControllerLouis))
    (Variables|Default|SetClicked_On_Down_Drawer true)
    (if (Rendering|IsVisible (Variables|Default|GetDefaultSceneRoot))
      (if (not (Variables|Default|GetHas%20Interact))
        (if (Variables|/Game/Dev_Louis/02_Blueprint/03_Player/BP_ThirdPersonPlayerController_Louis.BP_ThirdPersonPlayerController_Louis_C|GetAllowInteractionWithWorld (CallFunction|GetPlayerControllerLouis))
          (Variables|Default|SetHas%20Interact true)
          (CallFunction|Activate))))))

(event OnInputTouchBegin(Up_Drower_Collider)
  (params (FingerIndex :type ETouchIndex%20Enum :default "Touch1") (TouchedComponent :type Primitive%20Component%20Object%20Reference))
  (if (Variables|/Game/Dev_Louis/02_Blueprint/03_Player/BP_ThirdPersonPlayerController_Louis.BP_ThirdPersonPlayerController_Louis_C|GetAllowInteraction (CallFunction|GetPlayerControllerLouis))
    (Variables|Default|SetClicked_On_Up_Drawer true)
    (if (Rendering|IsVisible (Variables|Default|GetDefaultSceneRoot))
      (if (not (Variables|Default|GetHas%20Interact))
        (if (Variables|/Game/Dev_Louis/02_Blueprint/03_Player/BP_ThirdPersonPlayerController_Louis.BP_ThirdPersonPlayerController_Louis_C|GetAllowInteractionWithWorld (CallFunction|GetPlayerControllerLouis))
          (Variables|Default|SetHas%20Interact true)
          (CallFunction|Activate))))))

(event Custom|Open_Drawer_Up
  (bind _progression (Timeline|Timeline PlayFromStart)
    (:Update
      (Transformation|SetRelativeLocation (Variables|Default|GetDresser_Drawer_Up) (Math|Vector|MakeVector (Math|Float|Lerp (Variables|Default|GetUp_Drawer_Close_Position) (Variables|Default|GetUp_Drawer_Open_Position) _progression) 0.0 0.0) true false))
    (:Finished
      (Variables|Default|SetHas%20Interact false)
      (Variables|Default|SetClicked_On_Up_Drawer false)
      (Transformation|SetRelativeLocation (Variables|Default|GetUp_Drower_Collider) "0.000000,0.000000,-100.000000" false true)
      (Variables|Default|SetDrawer_Up_Is_Open true)
      (CallFunction|PreSave)
      (Default|IncrementActions (Variables|/Game/Dev_Louis/02_Blueprint/03_Player/BP_ThirdPersonPlayerController_Louis.BP_ThirdPersonPlayerController_Louis_C|GetEnemy (CallFunction|GetPlayerControllerLouis)) 1))))

(event Custom|Open_Drawer_Down
  (bind _progression (Timeline|Timeline_0 PlayFromStart)
    (:Update
      (Transformation|SetRelativeLocation (Variables|Default|GetDresser_Drawer_Down) (Math|Vector|MakeVector (Math|Float|Lerp (Variables|Default|GetDown_Drawer_Close_Position) (Variables|Default|GetDown_Drawer_Open_Position) _progression) 0.0 0.0) true false))
    (:Finished
      (Variables|Default|SetHas%20Interact false)
      (Variables|Default|SetClicked_On_Down_Drawer false)
      (Transformation|SetRelativeLocation (Variables|Default|GetDown_Drower_Collider) "0.000000,0.000000,-100.000000" false true)
      (Variables|Default|SetDrawer_Down_Is_Open true)
      (CallFunction|PreSave)
      (Default|IncrementActions (Variables|/Game/Dev_Louis/02_Blueprint/03_Player/BP_ThirdPersonPlayerController_Louis.BP_ThirdPersonPlayerController_Louis_C|GetEnemy (CallFunction|GetPlayerControllerLouis)) 1))))

(event EventActivate
  (Variables|/Game/Dev_Louis/02_Blueprint/03_Player/BP_ThirdPersonPlayerController_Louis.BP_ThirdPersonPlayerController_Louis_C|SetAllowInteraction (CallFunction|GetPlayerControllerLouis) false)
  (if (Variables|Default|GetHas%20Interact)
    (if (Variables|Default|GetPlayer_Is_In_Range)
      (Default|StartAnimationMontage (CallFunction|GetPlayerControllerLouis) "/Game/Art_Dev_Common/Animations/Player/AM_Player_Interaction.AM_Player_Interaction")
      (if (Variables|Default|GetClicked_On_Up_Drawer)
        (CallFunction|OpenDrawerUp)
        (Variables|/Game/Dev_Louis/02_Blueprint/03_Player/BP_ThirdPersonPlayerController_Louis.BP_ThirdPersonPlayerController_Louis_C|SetAllowInteraction (CallFunction|GetPlayerControllerLouis) true :!label _label)
        (elif (Variables|Default|GetClicked_On_Down_Drawer)
          (CallFunction|OpenDrawerDown)
          (goto _label)))
      (else
        (CallFunction|TriggerMovement)
        (goto _label)))))

(event EventPreSave
  (Variables|Default|SetObject_Value (+ (Math|Integer|SelectInt 1 0 (Variables|Default|GetDrawer_Up_Is_Open)) (Math|Integer|SelectInt 10 0 (Variables|Default|GetDrawer_Down_Is_Open))))
  (CallFunction|TempSave))

(event EventAfterLoad
  (params (Int_Value :type Integer))
  (if (not (== Int_Value 0))
    (if (== Int_Value 1)
      (Variables|Default|SetDrawer_Up_Is_Open true)
      (CallFunction|OpenDrawerUp)
      (elif (== Int_Value 10)
        (Variables|Default|SetDrawer_Down_Is_Open true)
        (CallFunction|OpenDrawerDown)
        (elif (== Int_Value 11)
          (Variables|Default|SetDrawer_Up_Is_Open true)
          (Variables|Default|SetDrawer_Down_Is_Open true)
          (CallFunction|OpenDrawerUp)
          (CallFunction|OpenDrawerDown))))))

(fn ConstructionScript
  (|CallParentFunction))