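; Savable interactable camera pickup that sets HaveCamera on the player controller when collected.
; A touch on the visible collider, if world interaction is allowed, calls Activate, which collects and hides the object when the player is in range.
; Otherwise it sends the player toward PlayerPosition, leaving the interaction pending.
; Activate triggers PreSave to store HaveCamera as an integer, and AfterLoad restores the flag, hiding the pickup if owned.
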(event OnInputTouchBegin(Collider)
  (params (FingerIndex :type ETouchIndex%20Enum :default "Touch1") (TouchedComponent :type Primitive%20Component%20Object%20Reference))
  (if (Rendering|IsVisible (Variables|Default|GetDefaultSceneRoot))
    (if (not (Variables|Default|GetHave_Interact))
      (if (Variables|/Game/Dev_Youenn/02_Blueprint/03_Player/BP_Player_Controller_Youenn.BP_Player_Controller_Youenn_C|GetAllow_To_Interact_Whis_World (CallFunction|GetPlayerControllerYouenn))
        (Variables|Default|SetHave_Interact true)
        (CallFunction|Activate)))))

(event EventPreSave
  (Variables|Default|SetObject_Value (Math|Integer|SelectInt 1 0 (Variables|/Game/Dev_Youenn/02_Blueprint/03_Player/BP_Player_Controller_Youenn.BP_Player_Controller_Youenn_C|GetHave_Camera (CallFunction|GetPlayerControllerYouenn))))
  (CallFunction|TempSave))

(event EventAfterLoad
  (params (Int_Value :type Integer))
  (bind _output_get (Variables|/Game/Dev_Youenn/02_Blueprint/03_Player/BP_Player_Controller_Youenn.BP_Player_Controller_Youenn_C|SetHave_Camera (CallFunction|GetPlayerControllerYouenn) (Utilities|Select :Index Int_Value :Option%200 false :Option%201 true)))
  (if _output_get
    (Rendering|SetVisibility (Variables|Default|GetDefaultSceneRoot) false true)))

(event EventActivate
  (if (Variables|Default|GetHave_Interact)
    (if (Variables|Default|GetPlayer_Is_In_Range)
      (Variables|/Game/Dev_Youenn/02_Blueprint/03_Player/BP_Player_Controller_Youenn.BP_Player_Controller_Youenn_C|SetHave_Camera (CallFunction|GetPlayerControllerYouenn) true)
      (Rendering|SetVisibility (Variables|Default|GetDefaultSceneRoot) false true)
      (Variables|Default|SetHave_Interact false)
      (else
        (Default|CallTargetMovement (CallFunction|GetPlayerControllerYouenn) (Transformation|GetActorLocation (Variables|Default|GetPlayer_Position)) (Variables|Default|GetPermission))))
    (CallFunction|PreSave)))

(fn ConstructionScript
  (|CallParentFunction))