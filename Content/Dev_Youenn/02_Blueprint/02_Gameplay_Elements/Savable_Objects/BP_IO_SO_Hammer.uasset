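; Savable interactable hammer pickup that grants the player the hammer when touched.
; A touch, gated by visibility and the controller's world-interaction flag, either collects it with a random pickup sound and hides it when in range, or triggers movement otherwise.
; Saving packs the controller's hammer and enchanted-hammer flags into one integer.
; Loading restores those flags from a positive value and sets the pickup's visibility accordingly.
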(event OnInputTouchBegin(Collider)
  (params (FingerIndex :type ETouchIndex%20Enum :default "Touch1") (TouchedComponent :type Primitive%20Component%20Object%20Reference))
  (if (Rendering|IsVisible (Variables|Default|GetDefaultSceneRoot))
    (if (not (Variables|Default|GetHas%20Interact))
      (if (Variables|/Game/Dev_Louis/02_Blueprint/03_Player/BP_ThirdPersonPlayerController_Louis.BP_ThirdPersonPlayerController_Louis_C|GetAllowInteractionWithWorld (CallFunction|GetPlayerControllerLouis))
        (Variables|Default|SetHas%20Interact true)
        (CallFunction|Activate)))))

(event EventActivate
  (if (Variables|Default|GetHas%20Interact)
    (if (Variables|Default|GetPlayer_Is_In_Range)
      (Audio|PlaySound2D (.OutItem (Utilities|Array|Random (Variables|Default|GetSoundsEffects))) 1.0 1.0 0.0 0 0)
      (Variables|/Game/Dev_Louis/02_Blueprint/03_Player/BP_ThirdPersonPlayerController_Louis.BP_ThirdPersonPlayerController_Louis_C|SetHaveHammer (CallFunction|GetPlayerControllerLouis) true)
      (Rendering|SetVisibility (Variables|Default|GetDefaultSceneRoot) false true)
      (Variables|Default|SetHas%20Interact false)
      (else
        (CallFunction|TriggerMovement)))
    (CallFunction|PreSave)))

(event EventPreSave
  (Variables|Default|SetObject_Value (+ (Math|Integer|SelectInt 1 0 (Variables|/Game/Dev_Louis/02_Blueprint/03_Player/BP_ThirdPersonPlayerController_Louis.BP_ThirdPersonPlayerController_Louis_C|GetHaveHammer (CallFunction|GetPlayerControllerLouis))) (Math|Integer|SelectInt 1 0 (Variables|/Game/Dev_Louis/02_Blueprint/03_Player/BP_ThirdPersonPlayerController_Louis.BP_ThirdPersonPlayerController_Louis_C|GetHaveEnchantHammer (CallFunction|GetPlayerControllerLouis)))))
  (CallFunction|TempSave))

(event EventAfterLoad
  (params (Int_Value :type Integer))
  (bind _asbp_third_person_player_controller_louis (CallFunction|GetPlayerControllerLouis))
  (bind _asbp_third_person_player_controller_louis_2 (CallFunction|GetPlayerControllerLouis))
  (if (> Int_Value 0)
    (if (> Int_Value 1)
      (bind _output_get (Variables|/Game/Dev_Louis/02_Blueprint/03_Player/BP_ThirdPersonPlayerController_Louis.BP_ThirdPersonPlayerController_Louis_C|SetHaveHammer _asbp_third_person_player_controller_louis_2 true))
      (Variables|/Game/Dev_Louis/02_Blueprint/03_Player/BP_ThirdPersonPlayerController_Louis.BP_ThirdPersonPlayerController_Louis_C|SetHaveEnchantHammer _asbp_third_person_player_controller_louis_2 _output_get)
      (else
        (Variables|/Game/Dev_Louis/02_Blueprint/03_Player/BP_ThirdPersonPlayerController_Louis.BP_ThirdPersonPlayerController_Louis_C|SetHaveHammer _asbp_third_person_player_controller_louis true)
        (Variables|/Game/Dev_Louis/02_Blueprint/03_Player/BP_ThirdPersonPlayerController_Louis.BP_ThirdPersonPlayerController_Louis_C|SetHaveEnchantHammer _asbp_third_person_player_controller_louis false)))
    (Rendering|SetVisibility (Variables|Default|GetDefaultSceneRoot) false true)
    (else
      (Rendering|SetVisibility (Variables|Default|GetDefaultSceneRoot) true true))))

(fn ConstructionScript
  (|CallParentFunction))