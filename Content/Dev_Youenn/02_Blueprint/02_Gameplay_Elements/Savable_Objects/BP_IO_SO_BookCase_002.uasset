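; Savable interactive bookcase with upper and lower drawers that open once each when tapped.
; A tap on a drawer collider locks player interaction and opens that drawer if the player is in range, otherwise it calls TriggerMovement.
; Timelines slide the drawer mesh, then shift its collider, save and increment the enemy's action count.
; Both states pack into one integer (tens upper, units lower), and loading replays the opening.
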(event OnInputTouchBegin(Drawer_Down_Collider)
  (params (FingerIndex :type ETouchIndex%20Enum :default "Touch1") (TouchedComponent :type Primitive%20Component%20Object%20Reference))
  (if (Variables|/Game/Dev_Louis/02_Blueprint/03_Player/BP_ThirdPersonPlayerController_Louis.BP_ThirdPersonPlayerController_Louis_C|GetAllowInteraction (CallFunction|GetPlayerControllerLouis))
    (Variables|//---HORIZONTALDOORDOWN---\\|SetClicked_On_Drawer_Down true)
    (if (Rendering|IsVisible (Variables|Default|GetDefaultSceneRoot))
      (if (not (Variables|Default|GetHas%20Interact))
        (if (Variables|/Game/Dev_Louis/02_Blueprint/03_Player/BP_ThirdPersonPlayerController_Louis.BP_ThirdPersonPlayerController_Louis_C|GetAllowInteractionWithWorld (CallFunction|GetPlayerControllerLouis))
          (Variables|Default|SetHas%20Interact true)
          (CallFunction|Activate))))))

(event OnInputTouchBegin(Drawer_Up_Collider)
  (params (FingerIndex :type ETouchIndex%20Enum :default "Touch1") (TouchedComponent :type Primitive%20Component%20Object%20Reference))
  (if (Variables|/Game/Dev_Louis/02_Blueprint/03_Player/BP_ThirdPersonPlayerController_Louis.BP_ThirdPersonPlayerController_Louis_C|GetAllowInteraction (CallFunction|GetPlayerControllerLouis))
    (Variables|//---HORIZONTALDOORUP---\\|SetClicked_On_Drawer_Up true)
    (if (Rendering|IsVisible (Variables|Default|GetDefaultSceneRoot))
      (if (not (Variables|Default|GetHas%20Interact))
        (if (Variables|/Game/Dev_Louis/02_Blueprint/03_Player/BP_ThirdPersonPlayerController_Louis.BP_ThirdPersonPlayerController_Louis_C|GetAllowInteractionWithWorld (CallFunction|GetPlayerControllerLouis))
          (Variables|Default|SetHas%20Interact true)
          (CallFunction|Activate))))))

(event Custom|Open_Up
  (bind _progression (Timeline|Timeline PlayFromStart)
    (:Update
      (Transformation|SetRelativeLocation (Variables|Default|GetAM_BookcaseDrawer_003) (Math|Vector|MakeVector (Math|Float|Lerp (Variables|//---HORIZONTALDOORUP---\\|GetDrawer_Up_Close_Position) (Variables|//---HORIZONTALDOORUP---\\|GetDrawer_Up_Open_Position) _progression) 0.0 0.0) false false))
    (:Finished
      (bind _output_get (Variables|//---HORIZONTALDOORUP---\\|SetClicked_On_Drawer_Up false))
      (Variables|Default|SetHas%20Interact _output_get)
      (Transformation|SetRelativeLocation (Variables|Default|GetDrawer_Up_Collider) "0.000000,0.000000,-100.000000" false true)
      (Variables|//---HORIZONTALDOORUP---\\|SetDrawer_Up_Is_Open true)
      (CallFunction|PreSave)
      (Default|IncrementActions (Variables|/Game/Dev_Louis/02_Blueprint/03_Player/BP_ThirdPersonPlayerController_Louis.BP_ThirdPersonPlayerController_Louis_C|GetEnemy (CallFunction|GetPlayerControllerLouis)) 1))))

(event Custom|Open_Down
  (bind _progression (Timeline|Timeline_0 PlayFromStart)
    (:Update
      (Transformation|SetRelativeLocation (Variables|Default|GetAM_BookcaseDrawer_001) (Math|Vector|MakeVector (Math|Float|Lerp (Variables|//---HORIZONTALDOORDOWN---\\|GetDrawer_Down_Close_Position) (Variables|//---HORIZONTALDOORDOWN---\\|GetDrawer_Down_Open_Position) _progression) 0.0 0.0) false false))
    (:Finished
      (bind _output_get (Variables|//---HORIZONTALDOORDOWN---\\|SetClicked_On_Drawer_Down false))
      (Variables|Default|SetHas%20Interact _output_get)
      (Transformation|SetRelativeLocation (Variables|Default|GetDrawer_Down_Collider) "0.000000,0.000000,-100.000000" false true)
      (Variables|//---HORIZONTALDOORDOWN---\\|SetDrawer_Down_Is_Open true)
      (CallFunction|PreSave)
      (Default|IncrementActions (Variables|/Game/Dev_Louis/02_Blueprint/03_Player/BP_ThirdPersonPlayerController_Louis.BP_ThirdPersonPlayerController_Louis_C|GetEnemy (CallFunction|GetPlayerControllerLouis)) 1))))

(event EventActivate
  (Variables|/Game/Dev_Louis/02_Blueprint/03_Player/BP_ThirdPersonPlayerController_Louis.BP_ThirdPersonPlayerController_Louis_C|SetAllowInteraction (CallFunction|GetPlayerControllerLouis) false)
  (if (Variables|Default|GetHas%20Interact)
    (if (Variables|Default|GetPlayer_Is_In_Range)
      (if (Variables|//---HORIZONTALDOORUP---\\|GetClicked_On_Drawer_Up)
        (CallFunction|OpenUp)
        (Variables|/Game/Dev_Louis/02_Blueprint/03_Player/BP_ThirdPersonPlayerController_Louis.BP_ThirdPersonPlayerController_Louis_C|SetAllowInteraction (CallFunction|GetPlayerControllerLouis) true :!label _label)
        (elif (Variables|//---HORIZONTALDOORDOWN---\\|GetClicked_On_Drawer_Down)
          (CallFunction|OpenDown)
          (goto _label)))
      (else
        (CallFunction|TriggerMovement)))))

(event EventPreSave
  (Variables|Default|SetObject_Value (+ (Math|Integer|SelectInt 10 0 (Variables|//---HORIZONTALDOORUP---\\|GetDrawer_Up_Is_Open)) (Math|Integer|SelectInt 1 0 (Variables|//---HORIZONTALDOORDOWN---\\|GetDrawer_Down_Is_Open))))
  (CallFunction|TempSave))

(event EventAfterLoad
  (params (Int_Value :type Integer))
  (if (== Int_Value 1)
    (Variables|//---HORIZONTALDOORDOWN---\\|SetDrawer_Down_Is_Open true)
    (CallFunction|OpenDown)
    (elif (== Int_Value 10)
      (Variables|//---HORIZONTALDOORUP---\\|SetDrawer_Up_Is_Open true)
      (CallFunction|OpenUp)
      (elif (== Int_Value 11)
        (bind _output_get (Variables|//---HORIZONTALDOORDOWN---\\|SetDrawer_Down_Is_Open true))
        (Variables|//---HORIZONTALDOORUP---\\|SetDrawer_Up_Is_Open _output_get)
        (CallFunction|OpenUp)
        (CallFunction|OpenDown)))))

(fn ConstructionScript
  (|CallParentFunction))