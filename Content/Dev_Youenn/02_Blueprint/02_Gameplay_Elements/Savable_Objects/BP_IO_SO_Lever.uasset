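; Savable touch-interactable lever that the player installs once they hold the lever item, then activates to unlock rooms.
; Touches trigger movement when out of range; in range, installing reveals the mesh, passes room data to the player controller and increments enemy actions.
; Activation rotates the lever and advances the map goal and dialogue.
; State is encoded as one integer (absent, installed, activated), saved on install and replayed on load.
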(event OnInputTouchBegin(Collider)
  (params (FingerIndex :type ETouchIndex%20Enum :default "Touch1") (TouchedComponent :type Primitive%20Component%20Object%20Reference))
  (if (not (Variables|Default|GetHas%20Interact))
    (if (Variables|/Game/Dev_Louis/02_Blueprint/03_Player/BP_ThirdPersonPlayerController_Louis.BP_ThirdPersonPlayerController_Louis_C|GetAllowInteractionWithWorld (CallFunction|GetPlayerControllerLouis))
      (Variables|Default|SetHas%20Interact true)
      (CallFunction|Activate))))

(event Custom|Activate_Lever
  (bind _asbp_third_person_player_controller_louis (CallFunction|GetPlayerControllerLouis))
  (Audio|PlaySound2D "/Game/Art_Dev_Common/SFX/SE_ActivateLever.SE_ActivateLever" 1.0 1.0 0.0 0 0)
  (Variables|Default|SetHas%20Interact false)
  (Variables|Default|SetHas_Been_Activated true)
  (Transformation|SetRelativeRotation (Variables|Default|GetLever) (Variables|Default|GetPosition_ON) false false)
  (Variables|/Game/Dev_Louis/02_Blueprint/03_Player/BP_ThirdPersonPlayerController_Louis.BP_ThirdPersonPlayerController_Louis_C|SetCurrentGoal _asbp_third_person_player_controller_louis 4)
  (Default|UpdateGoal (Variables|/Game/Dev_Louis/02_Blueprint/03_Player/BP_ThirdPersonPlayerController_Louis.BP_ThirdPersonPlayerController_Louis_C|GetMap _asbp_third_person_player_controller_louis))
  (Default|CharacterTalks (Variables|/Game/Dev_Louis/02_Blueprint/03_Player/BP_ThirdPersonPlayerController_Louis.BP_ThirdPersonPlayerController_Louis_C|GetMap _asbp_third_person_player_controller_louis) 8))

(event Custom|Install_Lever
  (Audio|PlaySound2D "/Game/Art_Dev_Common/SFX/SE_Clic_02.SE_Clic_02" 1.0 1.0 0.0 0 0)
  (Rendering|SetVisibility (Variables|Default|GetLever) true true)
  (Variables|Default|SetLever_Installed true)
  (Variables|Default|SetHas%20Interact false)
  (CallFunction|PreSave)
  (Default|IncrementActions (Variables|/Game/Dev_Louis/02_Blueprint/03_Player/BP_ThirdPersonPlayerController_Louis.BP_ThirdPersonPlayerController_Louis_C|GetEnemy (CallFunction|GetPlayerControllerLouis)) 1))

(event EventActivate
  (bind _asbp_third_person_player_controller_louis (CallFunction|GetPlayerControllerLouis))
  (bind _asbp_third_person_player_controller_louis_2 (CallFunction|GetPlayerControllerLouis))
  (if (Variables|/Game/Dev_Louis/02_Blueprint/03_Player/BP_ThirdPersonPlayerController_Louis.BP_ThirdPersonPlayerController_Louis_C|GetHaveLever (CallFunction|GetPlayerControllerLouis))
    (if (Variables|Default|GetLever_Installed)
      (if (Variables|Default|GetPlayer_Is_In_Range)
        (if (not (Variables|Default|GetHas_Been_Activated))
          (CallFunction|ActivateLever)
          (Default|UnlockRooms _asbp_third_person_player_controller_louis_2)
          (Variables|/Game/Dev_Louis/02_Blueprint/03_Player/BP_ThirdPersonPlayerController_Louis.BP_ThirdPersonPlayerController_Louis_C|SetHasUnlockedRooms _asbp_third_person_player_controller_louis_2 true))
        (else
          (CallFunction|TriggerMovement :!label _label)))
      (elif (Variables|Default|GetPlayer_Is_In_Range)
        (CallFunction|InstallLever)
        (Variables|/Game/Dev_Louis/02_Blueprint/03_Player/BP_ThirdPersonPlayerController_Louis.BP_ThirdPersonPlayerController_Louis_C|SetUnlockedRooms _asbp_third_person_player_controller_louis (Variables|Default|GetUnlockedRooms))
        (Variables|/Game/Dev_Louis/02_Blueprint/03_Player/BP_ThirdPersonPlayerController_Louis.BP_ThirdPersonPlayerController_Louis_C|SetConnectedRooms _asbp_third_person_player_controller_louis (Variables|Default|GetConnectedRooms))
        (else
          (goto _label))))
    (else
      (Variables|Default|SetHas%20Interact false))))

(event EventPreSave
  (Variables|Default|SetObject_Value (+ (Math|Integer|SelectInt 1 0 (Variables|Default|GetHas_Been_Activated)) (Math|Integer|SelectInt 1 0 (Variables|Default|GetLever_Installed))))
  (CallFunction|TempSave))

(event EventAfterLoad
  (params (Int_Value :type Integer))
  (if (> Int_Value 0)
    (if (> Int_Value 1)
      (bind _output_get (Variables|Default|SetLever_Installed true))
      (Variables|Default|SetHas_Been_Activated _output_get)
      (CallFunction|ActivateLever)
      (else
        (Variables|Default|SetLever_Installed true)
        (Variables|Default|SetHas_Been_Activated false)
        (CallFunction|InstallLever)))
    (else
      (Rendering|SetVisibility (Variables|Default|GetLever) false false))))

(fn ConstructionScript)