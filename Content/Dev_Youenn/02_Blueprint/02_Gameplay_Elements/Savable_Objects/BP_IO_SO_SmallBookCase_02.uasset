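; Savable interactive small bookcase whose doors the player opens by touch.
; A touch calls Activate, which triggers movement if the player is out of range, otherwise plays an interaction montage and sound, then opens the doors.
; A timeline lerps both door yaws, then lowers the collider, saves the open state as an integer and increments enemy actions.
; AfterLoad replays the opening for saved open doors.
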(event OnInputTouchBegin(Doors_Collider)
  (params (FingerIndex :type ETouchIndex%20Enum :default "Touch1") (TouchedComponent :type Primitive%20Component%20Object%20Reference))
  (if (Variables|/Game/Dev_Louis/02_Blueprint/03_Player/BP_ThirdPersonPlayerController_Louis.BP_ThirdPersonPlayerController_Louis_C|GetAllowInteraction (CallFunction|GetPlayerControllerLouis))
    (Variables|//---DOORS---\\|SetClicked_On_Doors true)
    (if (Rendering|IsVisible (Variables|Default|GetDefaultSceneRoot))
      (if (not (Variables|Default|GetHas%20Interact))
        (if (Variables|/Game/Dev_Louis/02_Blueprint/03_Player/BP_ThirdPersonPlayerController_Louis.BP_ThirdPersonPlayerController_Louis_C|GetAllowInteractionWithWorld (CallFunction|GetPlayerControllerLouis))
          (Variables|Default|SetHas%20Interact true)
          (CallFunction|Activate))))))

(event Custom|Open_Door
  (Variables|//---DOORS---\\|SetDoors_Is_Open true)
  (bind _progression (Timeline|T_Doors_Opening PlayFromStart)
    (:Update
      (Transformation|SetRelativeRotation (Variables|Default|GetRight_Door) (Math|Rotator|MakeRotator 0.0 0.0 (Math|Float|Lerp (Variables|//---DOORS---\\|GetRight_R_Doors_Close_Position) (Variables|//---DOORS---\\|GetRight_R_Doors_Open_Position) _progression)) false false)
      (Transformation|SetRelativeRotation (Variables|Default|GetLeft_Door) (Math|Rotator|MakeRotator 0.0 0.0 (Math|Float|Lerp (Variables|//---DOORS---\\|GetRight_L_Doors_Close_Position) (Variables|//---DOORS---\\|GetRight_L_Doors_Open_Position) _progression)) false false))
    (:Finished
      (bind _output_get (Variables|//---DOORS---\\|SetClicked_On_Doors false))
      (Variables|Default|SetHas%20Interact _output_get)
      (Transformation|SetRelativeLocation (Variables|Default|GetDoors_Collider) "0.000000,0.000000,-100.000000" false true)
      (CallFunction|PreSave)
      (Default|IncrementActions (Variables|/Game/Dev_Louis/02_Blueprint/03_Player/BP_ThirdPersonPlayerController_Louis.BP_ThirdPersonPlayerController_Louis_C|GetEnemy (CallFunction|GetPlayerControllerLouis)) 1))))

(event EventActivate
  (Variables|/Game/Dev_Louis/02_Blueprint/03_Player/BP_ThirdPersonPlayerController_Louis.BP_ThirdPersonPlayerController_Louis_C|SetAllowInteraction (CallFunction|GetPlayerControllerLouis) false)
  (if (Variables|Default|GetHas%20Interact)
    (if (Variables|Default|GetPlayer_Is_In_Range)
      (Default|PlayAnimationMontage (CallFunction|GetPlayerControllerLouis) "/Game/Art_Dev_Common/Animations/Player/AM_Player_Interaction.AM_Player_Interaction")
      (if (Variables|//---DOORS---\\|GetClicked_On_Doors)
        (Audio|PlaySound2D (.OutItem (Utilities|Array|Random (Variables|Default|GetSoundsEffects))) 1.0 1.0 0.0 0 0)
        (CallFunction|OpenDoor)
        (Variables|/Game/Dev_Louis/02_Blueprint/03_Player/BP_ThirdPersonPlayerController_Louis.BP_ThirdPersonPlayerController_Louis_C|SetAllowInteraction (CallFunction|GetPlayerControllerLouis) true :!label _label))
      (else
        (CallFunction|TriggerMovement)
        (goto _label)))))

(event EventPreSave
  (Variables|Default|SetObject_Value (Math|Integer|SelectInt 1 0 (Variables|//---DOORS---\\|GetDoors_Is_Open)))
  (CallFunction|TempSave))

(event EventAfterLoad
  (params (Int_Value :type Integer))
  (if (== Int_Value 1)
    (CallFunction|OpenDoor)
    (Variables|//---DOORS---\\|SetDoors_Is_Open true)))

(fn ConstructionScript
  (|CallParentFunction))