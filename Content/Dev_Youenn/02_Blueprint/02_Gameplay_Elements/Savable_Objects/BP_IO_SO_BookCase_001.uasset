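; Savable interactable bookcase with three horizontal doors that open on touch and stay open.
; A touch flags the door, then Activate opens it if the player is in range or otherwise triggers movement.
; Timelines rotate each door, then shift its companion component away, save and increment the enemy's action count.
; Door states pack into one decimal-digit integer, which AfterLoad decodes by replaying the same open events.
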(event OnInputTouchBegin(Horizontal_Door_Down)
  (params (FingerIndex :type ETouchIndex%20Enum :default "Touch1") (TouchedComponent :type Primitive%20Component%20Object%20Reference))
  (if (Variables|/Game/Dev_Louis/02_Blueprint/03_Player/BP_ThirdPersonPlayerController_Louis.BP_ThirdPersonPlayerController_Louis_C|GetAllowInteraction (CallFunction|GetPlayerControllerLouis))
    (Variables|//---HORIZONTALDOORDOWN---\\|SetClicked_On_Horizontal_Door_Down true)
    (if (Rendering|IsVisible (Variables|Default|GetDefaultSceneRoot))
      (if (not (Variables|Default|GetHas%20Interact))
        (if (Variables|/Game/Dev_Louis/02_Blueprint/03_Player/BP_ThirdPersonPlayerController_Louis.BP_ThirdPersonPlayerController_Louis_C|GetAllowInteractionWithWorld (CallFunction|GetPlayerControllerLouis))
          (Variables|Default|SetHas%20Interact true)
          (CallFunction|Activate))))))

(event OnInputTouchBegin(Horizontal_Door_Middle)
  (params (FingerIndex :type ETouchIndex%20Enum :default "Touch1") (TouchedComponent :type Primitive%20Component%20Object%20Reference))
  (if (Variables|/Game/Dev_Louis/02_Blueprint/03_Player/BP_ThirdPersonPlayerController_Louis.BP_ThirdPersonPlayerController_Louis_C|GetAllowInteraction (CallFunction|GetPlayerControllerLouis))
    (Variables|//---HORIZONTALDOORMIDDLE---\\|SetClicked_On_Horizontal_Door_Middle true)
    (if (Rendering|IsVisible (Variables|Default|GetDefaultSceneRoot))
      (if (not (Variables|Default|GetHas%20Interact))
        (if (Variables|/Game/Dev_Louis/02_Blueprint/03_Player/BP_ThirdPersonPlayerController_Louis.BP_ThirdPersonPlayerController_Louis_C|GetAllowInteractionWithWorld (CallFunction|GetPlayerControllerLouis))
          (Variables|Default|SetHas%20Interact true)
          (CallFunction|Activate))))))

(event OnInputTouchBegin(Horizontal_Door_Up)
  (params (FingerIndex :type ETouchIndex%20Enum :default "Touch1") (TouchedComponent :type Primitive%20Component%20Object%20Reference))
  (if (Variables|/Game/Dev_Louis/02_Blueprint/03_Player/BP_ThirdPersonPlayerController_Louis.BP_ThirdPersonPlayerController_Louis_C|GetAllowInteraction (CallFunction|GetPlayerControllerLouis))
    (Variables|//---HORIZONTALDOORUP---\\|SetClicked_On_Horizontal_Door_Up true)
    (if (Rendering|IsVisible (Variables|Default|GetDefaultSceneRoot))
      (if (not (Variables|Default|GetHas%20Interact))
        (if (Variables|/Game/Dev_Louis/02_Blueprint/03_Player/BP_ThirdPersonPlayerController_Louis.BP_ThirdPersonPlayerController_Louis_C|GetAllowInteractionWithWorld (CallFunction|GetPlayerControllerLouis))
          (Variables|Default|SetHas%20Interact true)
          (CallFunction|Activate))))))

(event Custom|Open_Middle_Door
  (bind _progression (Timeline|Timeline_0 PlayFromStart)
    (:Update
      (Transformation|SetRelativeRotation (Variables|Default|GetSMHorizontal_Door_Middle) (Math|Rotator|MakeRotator 0.0 (Math|Float|Lerp (Variables|//---HORIZONTALDOORMIDDLE---\\|GetHorizontal_Door_Middle_Close_Position) (Variables|//---HORIZONTALDOORMIDDLE---\\|GetHorizontal_Door_Middle_Open_Position) _progression) 0.0) false false))
    (:Finished
      (bind _output_get (Variables|//---HORIZONTALDOORMIDDLE---\\|SetClicked_On_Horizontal_Door_Middle false))
      (Variables|Default|SetHas%20Interact _output_get)
      (Transformation|SetRelativeLocation (Variables|Default|GetHorizontal_Door_Middle) "0.000000,0.000000,-100.000000" false true)
      (Variables|//---HORIZONTALDOORMIDDLE---\\|SetMiddle_Door_Is_Open true)
      (CallFunction|PreSave)
      (Default|IncrementActions (Variables|/Game/Dev_Louis/02_Blueprint/03_Player/BP_ThirdPersonPlayerController_Louis.BP_ThirdPersonPlayerController_Louis_C|GetEnemy (CallFunction|GetPlayerControllerLouis)) 1))))

(event Custom|Open_Top_Door
  (bind _progression (Timeline|Timeline PlayFromStart)
    (:Update
      (Transformation|SetRelativeRotation (Variables|Default|GetSM_Horizontal_Door_Up) (Math|Rotator|MakeRotator 0.0 (Math|Float|Lerp (Variables|//---HORIZONTALDOORUP---\\|GetHorizontal_Door_Up_Close_Position) (Variables|//---HORIZONTALDOORUP---\\|GetHorizontal_Door_Up_Open_Position) _progression) 0.0) false false))
    (:Finished
      (bind _output_get (Variables|//---HORIZONTALDOORUP---\\|SetClicked_On_Horizontal_Door_Up false))
      (Variables|Default|SetHas%20Interact _output_get)
      (Transformation|SetRelativeLocation (Variables|Default|GetHorizontal_Door_Up) "0.000000,0.000000,-100.000000" false true)
      (Variables|//---HORIZONTALDOORUP---\\|SetTop_Door_Is_Open true)
      (CallFunction|PreSave)
      (Default|IncrementActions (Variables|/Game/Dev_Louis/02_Blueprint/03_Player/BP_ThirdPersonPlayerController_Louis.BP_ThirdPersonPlayerController_Louis_C|GetEnemy (CallFunction|GetPlayerControllerLouis)) 1))))

(event Custom|Open_Bottom_Door
  (bind _progression (Timeline|Timeline_1 PlayFromStart)
    (:Update
      (Transformation|SetRelativeRotation (Variables|Default|GetSM_Horizontal_Door_Down) (Math|Rotator|MakeRotator 0.0 (Math|Float|Lerp (Variables|//---HORIZONTALDOORDOWN---\\|GetHorizontal_Door_Down_Close_Position) (Variables|//---HORIZONTALDOORDOWN---\\|GetHorizontal_Door_Down_Open_Position) _progression) 0.0) false false))
    (:Finished
      (bind _output_get (Variables|//---HORIZONTALDOORDOWN---\\|SetClicked_On_Horizontal_Door_Down false))
      (Variables|Default|SetHas%20Interact _output_get)
      (Transformation|SetRelativeLocation (Variables|Default|GetHorizontal_Door_Down) "0.000000,0.000000,-100.000000" false true)
      (Variables|//---HORIZONTALDOORDOWN---\\|SetBottom_Door_Is_Open true)
      (CallFunction|PreSave)
      (Default|IncrementActions (Variables|/Game/Dev_Louis/02_Blueprint/03_Player/BP_ThirdPersonPlayerController_Louis.BP_ThirdPersonPlayerController_Louis_C|GetEnemy (CallFunction|GetPlayerControllerLouis)) 1))))

(event EventActivate
  (Variables|/Game/Dev_Louis/02_Blueprint/03_Player/BP_ThirdPersonPlayerController_Louis.BP_ThirdPersonPlayerController_Louis_C|SetAllowInteraction (CallFunction|GetPlayerControllerLouis) false)
  (if (Variables|Default|GetHas%20Interact)
    (if (Variables|Default|GetPlayer_Is_In_Range)
      (if (Variables|//---HORIZONTALDOORUP---\\|GetClicked_On_Horizontal_Door_Up)
        (CallFunction|OpenTopDoor)
        (Variables|/Game/Dev_Louis/02_Blueprint/03_Player/BP_ThirdPersonPlayerController_Louis.BP_ThirdPersonPlayerController_Louis_C|SetAllowInteraction (CallFunction|GetPlayerControllerLouis) true :!label _label)
        (elif (Variables|//---HORIZONTALDOORMIDDLE---\\|GetClicked_On_Horizontal_Door_Middle)
          (CallFunction|OpenMiddleDoor)
          (goto _label)
          (elif (Variables|//---HORIZONTALDOORDOWN---\\|GetClicked_On_Horizontal_Door_Down)
            (CallFunction|OpenBottomDoor)
            (goto _label))))
      (else
        (CallFunction|TriggerMovement)))))

(event EventPreSave
  (Variables|Default|SetObject_Value (+ (Math|Integer|SelectInt 100 0 (Variables|//---HORIZONTALDOORUP---\\|GetTop_Door_Is_Open)) (Math|Integer|SelectInt 10 0 (Variables|//---HORIZONTALDOORMIDDLE---\\|GetMiddle_Door_Is_Open)) (Math|Integer|SelectInt 1 0 (Variables|//---HORIZONTALDOORDOWN---\\|GetBottom_Door_Is_Open))))
  (CallFunction|TempSave))

(event EventAfterLoad
  (params (Int_Value :type Integer))
  (if (not (== Int_Value 0))
    (if (== Int_Value 1)
      (CallFunction|OpenBottomDoor)
      (Variables|//---HORIZONTALDOORDOWN---\\|SetClicked_On_Horizontal_Door_Down true)
      (elif (== Int_Value 10)
        (CallFunction|OpenMiddleDoor)
        (Variables|//---HORIZONTALDOORMIDDLE---\\|SetClicked_On_Horizontal_Door_Middle true)
        (elif (== Int_Value 11)
          (CallFunction|OpenBottomDoor)
          (CallFunction|OpenMiddleDoor)
          (bind _output_get (Variables|//---HORIZONTALDOORDOWN---\\|SetClicked_On_Horizontal_Door_Down true))
          (Variables|//---HORIZONTALDOORMIDDLE---\\|SetClicked_On_Horizontal_Door_Middle _output_get)
          (elif (== Int_Value 100)
            (CallFunction|OpenTopDoor)
            (Variables|//---HORIZONTALDOORUP---\\|SetClicked_On_Horizontal_Door_Up true)
            (elif (== Int_Value 101)
              (CallFunction|OpenTopDoor)
              (CallFunction|OpenBottomDoor)
              (bind _output_get_2 (Variables|//---HORIZONTALDOORUP---\\|SetClicked_On_Horizontal_Door_Up true))
              (Variables|//---HORIZONTALDOORDOWN---\\|SetClicked_On_Horizontal_Door_Down _output_get_2)
              (elif (== Int_Value 110)
                (CallFunction|OpenTopDoor)
                (CallFunction|OpenMiddleDoor)
                (bind _output_get_3 (Variables|//---HORIZONTALDOORUP---\\|SetClicked_On_Horizontal_Door_Up true))
                (Variables|//---HORIZONTALDOORMIDDLE---\\|SetClicked_On_Horizontal_Door_Middle _output_get_3)
                (elif (== Int_Value 111)
                  (CallFunction|OpenTopDoor)
                  (CallFunction|OpenMiddleDoor)
                  (CallFunction|OpenBottomDoor)
                  (bind _output_get_4 (Variables|//---HORIZONTALDOORUP---\\|SetClicked_On_Horizontal_Door_Up true))
                  (bind _output_get_5 (Variables|//---HORIZONTALDOORMIDDLE---\\|SetClicked_On_Horizontal_Door_Middle _output_get_4))
                  (Variables|//---HORIZONTALDOORDOWN---\\|SetClicked_On_Horizontal_Door_Down _output_get_5))))))))))

(fn ConstructionScript
  (|CallParentFunction))