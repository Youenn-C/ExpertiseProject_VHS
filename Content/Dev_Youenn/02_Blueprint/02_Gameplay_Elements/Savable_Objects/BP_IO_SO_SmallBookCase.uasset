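; Savable small bookcase whose doors and two drawers the player opens by touch.
; Touched colliders set a flag and call Activate, which opens that part if the player is in range, otherwise triggers movement.
; Timelines animate each opening, then drop its collider and increment the enemy's action count.
; Open states pack into decimal-digit flags, saved only when doors finish opening; AfterLoad decodes them by replaying the openings.
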(event OnInputTouchBegin(Up_Drower_Collider)
  (params (FingerIndex :type ETouchIndex%20Enum :default "Touch1") (TouchedComponent :type Primitive%20Component%20Object%20Reference))
  (if (Variables|/Game/Dev_Louis/02_Blueprint/03_Player/BP_ThirdPersonPlayerController_Louis.BP_ThirdPersonPlayerController_Louis_C|GetAllowInteraction (CallFunction|GetPlayerControllerLouis))
    (Variables|//---UPDRAWERS---\\|SetClicked_On_Up_Drower true)
    (if (Rendering|IsVisible (Variables|Default|GetDefaultSceneRoot))
      (if (not (Variables|Default|GetHas%20Interact))
        (if (Variables|/Game/Dev_Louis/02_Blueprint/03_Player/BP_ThirdPersonPlayerController_Louis.BP_ThirdPersonPlayerController_Louis_C|GetAllowInteractionWithWorld (CallFunction|GetPlayerControllerLouis))
          (Variables|Default|SetHas%20Interact true)
          (CallFunction|Activate))))))

(event OnInputTouchBegin(Down_Drower_Collider)
  (params (FingerIndex :type ETouchIndex%20Enum :default "Touch1") (TouchedComponent :type Primitive%20Component%20Object%20Reference))
  (if (Variables|/Game/Dev_Louis/02_Blueprint/03_Player/BP_ThirdPersonPlayerController_Louis.BP_ThirdPersonPlayerController_Louis_C|GetAllowInteraction (CallFunction|GetPlayerControllerLouis))
    (Variables|//---DOWNDRAWERS---\\|SetClicked_On_Down_Drower true)
    (if (Rendering|IsVisible (Variables|Default|GetDefaultSceneRoot))
      (if (not (Variables|Default|GetHas%20Interact))
        (if (Variables|/Game/Dev_Louis/02_Blueprint/03_Player/BP_ThirdPersonPlayerController_Louis.BP_ThirdPersonPlayerController_Louis_C|GetAllowInteractionWithWorld (CallFunction|GetPlayerControllerLouis))
          (Variables|Default|SetHas%20Interact true)
          (CallFunction|Activate))))))

(event OnInputTouchBegin(Doors_Collider)
  (params (FingerIndex :type ETouchIndex%20Enum :default "Touch1") (TouchedComponent :type Primitive%20Component%20Object%20Reference))
  (if (Variables|/Game/Dev_Louis/02_Blueprint/03_Player/BP_ThirdPersonPlayerController_Louis.BP_ThirdPersonPlayerController_Louis_C|GetAllowInteraction (CallFunction|GetPlayerControllerLouis))
    (Variables|//---DOORS---\\|SetClicked_On_Doors true)
    (if (Rendering|IsVisible (Variables|Default|GetDefaultSceneRoot))
      (if (not (Variables|Default|GetHas%20Interact))
        (if (Variables|/Game/Dev_Louis/02_Blueprint/03_Player/BP_ThirdPersonPlayerController_Louis.BP_ThirdPersonPlayerController_Louis_C|GetAllowInteractionWithWorld (CallFunction|GetPlayerControllerLouis))
          (Variables|Default|SetHas%20Interact true)
          (CallFunction|Activate))))))

(event Custom|Open_Door
  (Variables|//---DOORS---\\|SetDoors_Is_Open true)
  (bind _progression (Timeline|T_Doors_Opening PlayFromStart)
    (:Update
      (Transformation|SetRelativeRotation (Variables|Default|GetRight_Door) (Math|Rotator|MakeRotator 0.0 0.0 (Math|Float|Lerp (Variables|//---DOORS---\\|GetRight_R_Doors_Close_Position) (Variables|//---DOORS---\\|GetRight_R_Doors_Open_Position) _progression)) false false)
      (Transformation|SetRelativeRotation (Variables|Default|GetLeft_Door) (Math|Rotator|MakeRotator 0.0 0.0 (Math|Float|Lerp (Variables|//---DOORS---\\|GetRight_L_Doors_Close_Position) (Variables|//---DOORS---\\|GetRight_L_Doors_Open_Position) _progression)) false false))
    (:Finished
      (bind _output_get (Variables|//---DOORS---\\|SetClicked_On_Doors false))
      (Variables|Default|SetHas%20Interact _output_get)
      (Transformation|SetRelativeLocation (Variables|Default|GetDoors_Collider) "0.000000,0.000000,-100.000000" false true)
      (CallFunction|PreSave)
      (Default|IncrementActions (Variables|/Game/Dev_Louis/02_Blueprint/03_Player/BP_ThirdPersonPlayerController_Louis.BP_ThirdPersonPlayerController_Louis_C|GetEnemy (CallFunction|GetPlayerControllerLouis)) 1))))

(event Custom|Open_Up_Drawer
  (Variables|//---UPDRAWERS---\\|SetUp_Drower_Is_Open true)
  (bind _progression (Timeline|T_Up_Drawer_Opening PlayFromStart)
    (:Update
      (Transformation|SetRelativeLocation (Variables|Default|GetUp_Drawer) (Math|Vector|MakeVector (Math|Float|Lerp (Variables|//---UPDRAWERS---\\|GetUp_Drawer_Close_Position) (Variables|//---DOWNDRAWERS---\\|GetUp_Drawer_Open_Position) _progression) 0.0 0.0) true false))
    (:Finished
      (bind _output_get (Variables|//---UPDRAWERS---\\|SetClicked_On_Up_Drower false))
      (Variables|Default|SetHas%20Interact _output_get)
      (Transformation|SetRelativeLocation (Variables|Default|GetUp_Drower_Collider) "0.000000,0.000000,-100.000000" false true)
      (Default|IncrementActions (Variables|/Game/Dev_Louis/02_Blueprint/03_Player/BP_ThirdPersonPlayerController_Louis.BP_ThirdPersonPlayerController_Louis_C|GetEnemy (CallFunction|GetPlayerControllerLouis)) 1))))

(event Custom|Open_Down_Drawer
  (Variables|//---DOWNDRAWERS---\\|SetDown_Drower_Is_Open true)
  (bind _progression (Timeline|T_Down_Drawer_Opening PlayFromStart)
    (:Update
      (Transformation|SetRelativeLocation (Variables|Default|GetDown_Drawer) (Math|Vector|MakeVector (Math|Float|Lerp (Variables|//---DOWNDRAWERS---\\|GetDown_Drawer_Close_Position) (Variables|//---DOWNDRAWERS---\\|GetDown_Drawer_Open_Position) _progression) 0.0 0.0) true false))
    (:Finished
      (bind _output_get (Variables|//---DOORS---\\|SetClicked_On_Doors false))
      (Variables|Default|SetHas%20Interact _output_get)
      (Transformation|SetRelativeLocation (Variables|Default|GetDown_Drower_Collider) "0.000000,0.000000,-100.000000" false true)
      (Default|IncrementActions (Variables|/Game/Dev_Louis/02_Blueprint/03_Player/BP_ThirdPersonPlayerController_Louis.BP_ThirdPersonPlayerController_Louis_C|GetEnemy (CallFunction|GetPlayerControllerLouis)) 1))))

(event EventActivate
  (Variables|/Game/Dev_Louis/02_Blueprint/03_Player/BP_ThirdPersonPlayerController_Louis.BP_ThirdPersonPlayerController_Louis_C|SetAllowInteraction (CallFunction|GetPlayerControllerLouis) false)
  (if (Variables|Default|GetHas%20Interact)
    (if (Variables|Default|GetPlayer_Is_In_Range)
      (if (Variables|//---DOORS---\\|GetClicked_On_Doors)
        (CallFunction|OpenDoor)
        (Variables|/Game/Dev_Louis/02_Blueprint/03_Player/BP_ThirdPersonPlayerController_Louis.BP_ThirdPersonPlayerController_Louis_C|SetAllowInteraction (CallFunction|GetPlayerControllerLouis) true :!label _label)
        (elif (Variables|//---UPDRAWERS---\\|GetClicked_On_Up_Drower)
          (CallFunction|OpenUpDrawer)
          (goto _label)
          (elif (Variables|//---DOWNDRAWERS---\\|GetClicked_On_Down_Drower)
            (CallFunction|OpenDownDrawer)
            (goto _label))))
      (else
        (CallFunction|TriggerMovement)))))

(event EventPreSave
  (Variables|Default|SetObject_Value (+ (Math|Integer|SelectInt 1 0 (Variables|//---DOORS---\\|GetDoors_Is_Open)) (Math|Integer|SelectInt 10 0 (Variables|//---UPDRAWERS---\\|GetUp_Drower_Is_Open)) (Math|Integer|SelectInt 100 0 (Variables|//---DOWNDRAWERS---\\|GetDown_Drower_Is_Open))))
  (CallFunction|TempSave))

(event EventAfterLoad
  (params (Int_Value :type Integer))
  (if (not (== Int_Value 0))
    (if (== Int_Value 1)
      (CallFunction|OpenDoor)
      (Variables|//---DOORS---\\|SetDoors_Is_Open true)
      (elif (== Int_Value 10)
        (CallFunction|OpenUpDrawer)
        (Variables|//---UPDRAWERS---\\|SetClicked_On_Up_Drower true)
        (elif (== Int_Value 11)
          (CallFunction|OpenDoor)
          (Variables|//---DOORS---\\|SetDoors_Is_Open true)
          (CallFunction|OpenUpDrawer)
          (Variables|//---UPDRAWERS---\\|SetClicked_On_Up_Drower true)
          (elif (== Int_Value 100)
            (CallFunction|OpenDownDrawer)
            (Variables|//---DOWNDRAWERS---\\|SetClicked_On_Down_Drower true)
            (elif (== Int_Value 101)
              (CallFunction|OpenDownDrawer)
              (Variables|//---DOWNDRAWERS---\\|SetClicked_On_Down_Drower true)
              (CallFunction|OpenDoor)
              (Variables|//---DOORS---\\|SetDoors_Is_Open true)
              (elif (== Int_Value 110)
                (CallFunction|OpenDownDrawer)
                (Variables|//---DOWNDRAWERS---\\|SetClicked_On_Down_Drower true)
                (CallFunction|OpenUpDrawer)
                (Variables|//---UPDRAWERS---\\|SetClicked_On_Up_Drower true)
                (elif (== Int_Value 111)
                  (CallFunction|OpenDownDrawer)
                  (Variables|//---DOWNDRAWERS---\\|SetClicked_On_Down_Drower true)
                  (CallFunction|OpenDoor)
                  (Variables|//---DOORS---\\|SetDoors_Is_Open true)
                  (CallFunction|OpenUpDrawer)
                  (Variables|//---UPDRAWERS---\\|SetClicked_On_Up_Drower true))))))))))

(fn ConstructionScript
  (|CallParentFunction))