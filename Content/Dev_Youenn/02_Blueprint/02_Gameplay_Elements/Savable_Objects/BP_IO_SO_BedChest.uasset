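; BP_IO_SO_BedChest is a touch-interactable, savable bed chest that opens once and restores its open state on load.
; A touch, gated by player controller flags, opens the chest when the player is in range, otherwise triggers movement.
; Opening rotates the lid via a timeline, then teleports the collider to a lowered position.
; The open flag is stored as an integer through TempSave, and AfterLoad replays the opening if set.
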(event OnInputTouchBegin(Collider)
  (params (FingerIndex :type ETouchIndex%20Enum :default "Touch1") (TouchedComponent :type Primitive%20Component%20Object%20Reference))
  (if (Variables|/Game/Dev_Youenn/02_Blueprint/03_Player/BP_Player_Controller_Youenn.BP_Player_Controller_Youenn_C|GetAllow%20Interaction (CallFunction|GetPlayerControllerYouenn))
    (if (not (Variables|Default|GetHave_Interact))
      (if (Variables|/Game/Dev_Youenn/02_Blueprint/03_Player/BP_Player_Controller_Youenn.BP_Player_Controller_Youenn_C|GetAllow_To_Interact_Whis_World (CallFunction|GetPlayerControllerYouenn))
        (Variables|Default|SetHave_Interact true)
        (CallFunction|Activate)))))

(event Custom|Open_Chest
  (Variables|Default|SetIs_Open true)
  (bind _progression (Timeline|Timeline PlayFromStart)
    (:Update
      (Transformation|SetRelativeRotation (Variables|Default|GetChest_Top) (Math|Rotator|MakeRotator 0.0 (Math|Float|Lerp (Variables|Default|GetChest_Top_Close_Position) (Variables|Default|GetChest_Top_Open_Position) _progression) 0.0) false false))
    (:Finished
      (Variables|Default|SetHave_Interact false)
      (Transformation|SetRelativeLocation (Variables|Default|GetCollider) "0.000000,0.000000,-100.000000" false true))))

(event EventActivate
  (Variables|/Game/Dev_Youenn/02_Blueprint/03_Player/BP_Player_Controller_Youenn.BP_Player_Controller_Youenn_C|SetAllow%20Interaction (CallFunction|GetPlayerControllerYouenn) false)
  (if (Variables|Default|GetHave_Interact)
    (if (Variables|Default|GetPlayer_Is_In_Range)
      (CallFunction|OpenChest)
      (Variables|/Game/Dev_Youenn/02_Blueprint/03_Player/BP_Player_Controller_Youenn.BP_Player_Controller_Youenn_C|SetAllow%20Interaction (CallFunction|GetPlayerControllerYouenn) true)
      (else
        (CallFunction|TriggerMovement)))
    (CallFunction|PreSave)))

(event EventPreSave
  (Variables|Default|SetObject_Value (Math|Integer|SelectInt 1 0 (Variables|Default|GetIs_Open)))
  (CallFunction|TempSave))

(event EventAfterLoad
  (params (Int_Value :type Integer))
  (bind _output_get (Variables|Default|SetIs_Open (Utilities|Select :Index Int_Value :Option%200 false :Option%201 true)))
  (if _output_get
    (CallFunction|OpenChest)))

(fn ConstructionScript
  (|CallParentFunction))