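; Savable interactive dresser whose two doors the player opens by touch.
; A touch on the doors collider plays the interaction montage and opens the doors if the player is in range, otherwise it triggers movement.
; A timeline swings both doors, then moves the collider away, saves and increments the enemy's action count.
; State saves as an integer, with the tens slot unused, and loading a value of 1 replays the opening.
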(event OnInputTouchBegin(Doors_Collider)
  (params (FingerIndex :type ETouchIndex%20Enum :default "Touch1") (TouchedComponent :type Primitive%20Component%20Object%20Reference))
  (if (Variables|/Game/Dev_Louis/02_Blueprint/03_Player/BP_ThirdPersonPlayerController_Louis.BP_ThirdPersonPlayerController_Louis_C|GetAllowInteraction (CallFunction|GetPlayerControllerLouis))
    (Variables|Default|SetClicked_On_Doors true)
    (if (Rendering|IsVisible (Variables|Default|GetDefaultSceneRoot))
      (if (not (Variables|Default|GetHas%20Interact))
        (if (Variables|/Game/Dev_Louis/02_Blueprint/03_Player/BP_ThirdPersonPlayerController_Louis.BP_ThirdPersonPlayerController_Louis_C|GetAllowInteractionWithWorld (CallFunction|GetPlayerControllerLouis))
          (Variables|Default|SetHas%20Interact true)
          (CallFunction|Activate))))))

(event Custom|Open_Doors
  (Variables|Default|SetDoors_Are_Open true)
  (bind _progression (Timeline|Timeline_0 PlayFromStart)
    (:Update
      (Transformation|SetRelativeRotation (Variables|Default|GetDresser_Right_Door) (Math|Rotator|MakeRotator 0.0 0.0 (Math|Float|Lerp (Variables|Default|GetRight_Door_Close_Position) (Variables|Default|GetRight_Door_Open_Position) _progression)) false false)
      (Transformation|SetRelativeRotation (Variables|Default|GetDresser_Left_Door) (Math|Rotator|MakeRotator 0.0 0.0 (Math|Float|Lerp (Variables|Default|GetLeft_Door_Close_Position) (Variables|Default|GetLeft_Door_Open_Position) _progression)) false false))
    (:Finished
      (bind _output_get (Variables|Default|SetClicked_On_Doors false))
      (Variables|Default|SetHas%20Interact _output_get)
      (Transformation|SetRelativeLocation (Variables|Default|GetDoors_Collider) "0.000000,0.000000,-100.000000" false true)
      (CallFunction|PreSave)
      (Default|IncrementActions (Variables|/Game/Dev_Louis/02_Blueprint/03_Player/BP_ThirdPersonPlayerController_Louis.BP_ThirdPersonPlayerController_Louis_C|GetEnemy (CallFunction|GetPlayerControllerLouis)) 1))))

(event EventActivate
  (Variables|/Game/Dev_Louis/02_Blueprint/03_Player/BP_ThirdPersonPlayerController_Louis.BP_ThirdPersonPlayerController_Louis_C|SetAllowInteraction (CallFunction|GetPlayerControllerLouis) false)
  (if (Variables|Default|GetHas%20Interact)
    (if (Variables|Default|GetPlayer_Is_In_Range)
      (Default|PlayAnimationMontage (CallFunction|GetPlayerControllerLouis) "/Game/Art_Dev_Common/Animations/Player/AM_Player_Interaction.AM_Player_Interaction")
      (if (Variables|Default|GetClicked_On_Doors)
        (CallFunction|OpenDoors)
        (Audio|PlaySound2D (.OutItem (Utilities|Array|Random (Variables|Default|GetSoundsEffects))) 1.0 1.0 0.0 0 0)
        (Variables|/Game/Dev_Louis/02_Blueprint/03_Player/BP_ThirdPersonPlayerController_Louis.BP_ThirdPersonPlayerController_Louis_C|SetAllowInteraction (CallFunction|GetPlayerControllerLouis) true :!label _label))
      (else
        (CallFunction|TriggerMovement)
        (goto _label)))))

(event EventPreSave
  (Variables|Default|SetObject_Value (+ (Math|Integer|SelectInt 1 0 (Variables|Default|GetDoors_Are_Open)) (Math|Integer|SelectInt 10 0 false)))
  (CallFunction|TempSave))

(event EventAfterLoad
  (params (Int_Value :type Integer))
  (if (not (== Int_Value 0))
    (if (== Int_Value 1)
      (Variables|Default|SetDoors_Are_Open true)
      (CallFunction|OpenDoors)
      (elif (not (== Int_Value 10))
        (if (== Int_Value 11)
          (Variables|Default|SetDoors_Are_Open true))))))

(fn ConstructionScript
  (|CallParentFunction))