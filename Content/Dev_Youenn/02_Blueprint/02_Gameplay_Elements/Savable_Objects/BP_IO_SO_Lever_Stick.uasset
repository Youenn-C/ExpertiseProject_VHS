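; Savable interactive pickup for a lever stick that the player collects by touch, flagging HaveLever on the player controller.
; A touch on the visible collider, when world interaction is allowed, increments the enemy's action count and calls Activate, which either collects and hides the stick in range or triggers movement.
; Activate then saves the flag as an integer and triggers character dialogue; AfterLoad restores the flag and hides collected sticks.
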(event OnInputTouchBegin(Collider)
  (params (FingerIndex :type ETouchIndex%20Enum :default "Touch1") (TouchedComponent :type Primitive%20Component%20Object%20Reference))
  (if (Rendering|IsVisible (Variables|Default|GetDefaultSceneRoot))
    (if (not (Variables|Default|GetHas%20Interact))
      (if (Variables|/Game/Dev_Louis/02_Blueprint/03_Player/BP_ThirdPersonPlayerController_Louis.BP_ThirdPersonPlayerController_Louis_C|GetAllowInteractionWithWorld (CallFunction|GetPlayerControllerLouis))
        (Variables|Default|SetHas%20Interact true)
        (CallFunction|Activate)
        (Default|IncrementActions (Variables|/Game/Dev_Louis/02_Blueprint/03_Player/BP_ThirdPersonPlayerController_Louis.BP_ThirdPersonPlayerController_Louis_C|GetEnemy (CallFunction|GetPlayerControllerLouis)) 1)))))

(event EventActivate
  (if (Variables|Default|GetHas%20Interact)
    (if (Variables|Default|GetPlayer_Is_In_Range)
      (Audio|PlaySound2D (.OutItem (Utilities|Array|Random (Variables|Default|GetSoundsEffects))) 1.0 1.0 0.0 0 0)
      (Variables|/Game/Dev_Louis/02_Blueprint/03_Player/BP_ThirdPersonPlayerController_Louis.BP_ThirdPersonPlayerController_Louis_C|SetHaveLever (CallFunction|GetPlayerControllerLouis) true)
      (Rendering|SetVisibility (Variables|Default|GetDefaultSceneRoot) false true)
      (Variables|Default|SetHas%20Interact false)
      (else
        (CallFunction|TriggerMovement)))
    (CallFunction|PreSave)
    (Default|CharacterTalks (Variables|/Game/Dev_Louis/02_Blueprint/03_Player/BP_ThirdPersonPlayerController_Louis.BP_ThirdPersonPlayerController_Louis_C|GetMap (CallFunction|GetPlayerControllerLouis)) 7)))

(event EventPreSave
  (Variables|Default|SetObject_Value (Math|Integer|SelectInt 1 0 (Variables|/Game/Dev_Louis/02_Blueprint/03_Player/BP_ThirdPersonPlayerController_Louis.BP_ThirdPersonPlayerController_Louis_C|GetHaveLever (CallFunction|GetPlayerControllerLouis))))
  (CallFunction|TempSave))

(event EventAfterLoad
  (params (Int_Value :type Integer))
  (bind _output_get (Variables|/Game/Dev_Louis/02_Blueprint/03_Player/BP_ThirdPersonPlayerController_Louis.BP_ThirdPersonPlayerController_Louis_C|SetHaveLever (CallFunction|GetPlayerControllerLouis) (Utilities|Select :Index Int_Value :Option%200 false :Option%201 true)))
  (if _output_get
    (Rendering|SetVisibility (Variables|Default|GetDefaultSceneRoot) false true)))

(fn ConstructionScript
  (|CallParentFunction))