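; Savable interactive fridge whose door the player opens by touch, with the open state kept through the save system.
; A touch passes the player controller's interaction checks, then opens the door if in range or triggers movement.
; Opening plays a random sound, lerps door yaw on a timeline, sinks the collider, saves and increments the enemy's action count.
; Loading an open state replays that whole sequence.
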(event OnInputTouchBegin(Collider)
  (params (FingerIndex :type ETouchIndex%20Enum :default "Touch1") (TouchedComponent :type Primitive%20Component%20Object%20Reference))
  (if (Variables|/Game/Dev_Louis/02_Blueprint/03_Player/BP_ThirdPersonPlayerController_Louis.BP_ThirdPersonPlayerController_Louis_C|GetAllowInteraction (CallFunction|GetPlayerControllerLouis))
    (if (not (Variables|Default|GetHas%20Interact))
      (if (Variables|/Game/Dev_Louis/02_Blueprint/03_Player/BP_ThirdPersonPlayerController_Louis.BP_ThirdPersonPlayerController_Louis_C|GetAllowInteractionWithWorld (CallFunction|GetPlayerControllerLouis))
        (Variables|Default|SetHas%20Interact true)
        (CallFunction|Activate)))))

(event Custom|Open_Door
  (Audio|PlaySound2D (.OutItem (Utilities|Array|Random (Variables|Default|GetSoundsEffects))) 1.0 1.0 0.0 0 0)
  (bind _progression (Timeline|Timeline PlayFromStart)
    (:Update
      (Transformation|SetRelativeRotation (Variables|Default|GetAM_FridgeDoor_001) (Math|Rotator|MakeRotator 0.0 0.0 (Math|Float|Lerp (Variables|//---DOORS---\\|GetDoor_Close_Position) (Variables|//---DOORS---\\|GetDoor_Open_Position) _progression)) false false))
    (:Finished
      (Variables|Default|SetHas%20Interact false)
      (Transformation|SetRelativeLocation (Variables|Default|GetCollider) "0.000000,0.000000,-200.000000" false true)
      (Variables|//---DOORS---\\|SetDoors_Is_Open true)
      (CallFunction|PreSave)
      (Default|IncrementActions (Variables|/Game/Dev_Louis/02_Blueprint/03_Player/BP_ThirdPersonPlayerController_Louis.BP_ThirdPersonPlayerController_Louis_C|GetEnemy (CallFunction|GetPlayerControllerLouis)) 1))))

(event EventActivate
  (Variables|/Game/Dev_Louis/02_Blueprint/03_Player/BP_ThirdPersonPlayerController_Louis.BP_ThirdPersonPlayerController_Louis_C|SetAllowInteraction (CallFunction|GetPlayerControllerLouis) false)
  (if (Variables|Default|GetHas%20Interact)
    (if (Variables|Default|GetPlayer_Is_In_Range)
      (CallFunction|OpenDoor)
      (else
        (CallFunction|TriggerMovement)))
    (Variables|/Game/Dev_Louis/02_Blueprint/03_Player/BP_ThirdPersonPlayerController_Louis.BP_ThirdPersonPlayerController_Louis_C|SetAllowInteraction (CallFunction|GetPlayerControllerLouis) true)))

(event EventPreSave
  (Variables|Default|SetObject_Value (Math|Integer|SelectInt 1 0 (Variables|//---DOORS---\\|GetDoors_Is_Open)))
  (CallFunction|TempSave))

(event EventAfterLoad
  (params (Int_Value :type Integer))
  (bind _output_get (Variables|//---DOORS---\\|SetDoors_Is_Open (Utilities|Select :Index Int_Value :Option%200 false :Option%201 true)))
  (if _output_get
    (CallFunction|OpenDoor)))

(fn ConstructionScript
  (|CallParentFunction))