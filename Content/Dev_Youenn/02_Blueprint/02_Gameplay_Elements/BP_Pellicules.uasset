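; BP_Pellicules is a clickable pickup that adds one pellicule to the player's count.
; Clicking its sphere calls Activate, which compares CurrentPellicules to MaxPellicules on the player controller from GetPlayerControllerYouenn.
; Below the maximum, it increments the count and destroys itself; otherwise it only prints a placeholder "Hello" message.
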(event OnClicked(Sphere)
  (params (TouchedComponent :type Primitive%20Component%20Object%20Reference) (ButtonPressed :type Key%20Structure :default "None"))
  (CallFunction|Activate))

(event EventActivate
  (bind _asbp_player_controller_youenn (CallFunction|GetPlayerControllerYouenn))
  (bind _asbp_player_controller_youenn_2 (CallFunction|GetPlayerControllerYouenn))
  (if (< (Variables|/Game/Dev_Youenn/02_Blueprint/03_Player/BP_Player_Controller_Youenn.BP_Player_Controller_Youenn_C|GetCurrent_Pellicules _asbp_player_controller_youenn) (Variables|/Game/Dev_Youenn/02_Blueprint/03_Player/BP_Player_Controller_Youenn.BP_Player_Controller_Youenn_C|GetMax_Pellicules _asbp_player_controller_youenn))
    (bind _result (Math|Integer|IncrementInt (Variables|/Game/Dev_Youenn/02_Blueprint/03_Player/BP_Player_Controller_Youenn.BP_Player_Controller_Youenn_C|GetCurrent_Pellicules _asbp_player_controller_youenn_2))
      (:%20%20
        (Variables|/Game/Dev_Youenn/02_Blueprint/03_Player/BP_Player_Controller_Youenn.BP_Player_Controller_Youenn_C|SetCurrent_Pellicules _asbp_player_controller_youenn_2 _result)
        (Actor|DestroyActor)))
    (else
      (Development|PrintString "Hello"))))

(fn ConstructionScript)