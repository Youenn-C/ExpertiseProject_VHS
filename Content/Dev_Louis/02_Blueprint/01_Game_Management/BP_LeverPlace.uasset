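; Touch-interactable lever socket where the player places a lever, then pulls it to unlock rooms.
; Touching the mesh requires a non-empty UnlockedRooms list on the player controller: the first touch swaps the material and flags the lever as placed, the next calls UnlockRooms and locks the socket.
; Each successful touch increments the enemy's action count, and on-screen French debug strings report placement, missing-lever and already-used states.
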(event OnInputTouchBegin(SM)
  (params (FingerIndex :type ETouchIndex%20Enum :default "Touch1") (TouchedComponent :type Primitive%20Component%20Object%20Reference))
  (bind _asbp_third_person_player_controller_louis (CallFunction|GetPlayerControllerLouis))
  (if (!= true (Variables|Default|GetAlreadyUsed))
    (if (Utilities|Array|IsNotEmpty (Variables|/Game/Dev_Louis/02_Blueprint/03_Player/BP_ThirdPersonPlayerController_Louis.BP_ThirdPersonPlayerController_Louis_C|GetUnlockedRooms _asbp_third_person_player_controller_louis))
      (if (Variables|/Game/Dev_Louis/02_Blueprint/03_Player/BP_ThirdPersonPlayerController_Louis.BP_ThirdPersonPlayerController_Louis_C|GetHasPlacedLever _asbp_third_person_player_controller_louis)
        (Default|UnlockRooms _asbp_third_person_player_controller_louis)
        (Variables|Default|SetAlreadyUsed true)
        (else
          (Rendering|Material|SetMaterial (Variables|Default|GetSM) 0 "/Engine/BasicShapes/BasicShapeMaterial.BasicShapeMaterial")
          (Development|PrintString "Levier placé. Toucher pour l'utiliser")
          (Variables|/Game/Dev_Louis/02_Blueprint/03_Player/BP_ThirdPersonPlayerController_Louis.BP_ThirdPersonPlayerController_Louis_C|SetHasPlacedLever _asbp_third_person_player_controller_louis true)))
      (Default|IncrementActions (Variables|/Game/Dev_Louis/02_Blueprint/03_Player/BP_ThirdPersonPlayerController_Louis.BP_ThirdPersonPlayerController_Louis_C|GetEnemy (CallFunction|GetPlayerControllerLouis)) 1)
      (else
        (Development|PrintString "Il faut d'abord récupérer le levier pour le poser ici")))
    (else
      (Development|PrintString "Le levier a déjà été utilisé"))))

(event Collision|EventActorBeginOverlap
  (params (OtherActor :type Actor%20Object%20Reference)))

(event EventTick
  (params (DeltaSeconds :type Float%20%28single-precision%29)))

(fn ConstructionScript)