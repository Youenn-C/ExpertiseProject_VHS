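; Interactive touch door that transfers the player between rooms, optionally starting hidden and locked until UnlockDoor.
; Touching either side sends the player to that side's target point or, if in range, opens it via timeline, then changes room and repositions the character.
; In Polaroid mode, touches instead spend a cartridge to print whether the door's room holds an enemy.
; Tick swaps the door material to highlight neighboring rooms during that mode.
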(event OnInputTouchBegin(TouchDetectorSideB)
  (params (FingerIndex :type ETouchIndex%20Enum :default "Touch1") (TouchedComponent :type Primitive%20Component%20Object%20Reference))
  (bind _asbp_third_person_player_controller_louis (CallFunction|GetPlayerControllerLouis))
  ;[0.15 0.15 0.15 0.5] Récupération de l'information du clic
  (if (Variables|/Game/Dev_Louis/02_Blueprint/03_Player/BP_ThirdPersonPlayerController_Louis.BP_ThirdPersonPlayerController_Louis_C|GetAllowInteraction (CallFunction|GetPlayerControllerLouis))
    (if (Variables|/Game/Dev_Louis/02_Blueprint/03_Player/BP_ThirdPersonPlayerController_Louis.BP_ThirdPersonPlayerController_Louis_C|GetIsUsingPolaroid (CallFunction|GetPlayerControllerLouis))
      (CallFunction|CheckEnemyinRoom)
      (elif (not (Variables|Default|GetHas%20Interact))
        (if (Variables|/Game/Dev_Louis/02_Blueprint/03_Player/BP_ThirdPersonPlayerController_Louis.BP_ThirdPersonPlayerController_Louis_C|GetAllowInteractionWithWorld _asbp_third_person_player_controller_louis)
          (Variables|Default|SetHas%20Interact true)
          (Variables|/Game/Dev_Louis/02_Blueprint/03_Player/BP_ThirdPersonPlayerController_Louis.BP_ThirdPersonPlayerController_Louis_C|SetAllowInteraction _asbp_third_person_player_controller_louis false)
          (CallFunction|Activate))))))

(event OnInputTouchBegin(TouchDetectorSideA)
  (params (FingerIndex :type ETouchIndex%20Enum :default "Touch1") (TouchedComponent :type Primitive%20Component%20Object%20Reference))
  (bind _asbp_third_person_player_controller_louis (CallFunction|GetPlayerControllerLouis))
  ;[0.15 0.15 0.15 0.5] Récupération de l'information du clic
  (if (not (Variables|Default|GetLockedDoor))
    (if (Variables|/Game/Dev_Louis/02_Blueprint/03_Player/BP_ThirdPersonPlayerController_Louis.BP_ThirdPersonPlayerController_Louis_C|GetAllowInteraction (CallFunction|GetPlayerControllerLouis))
      (Variables|//--BOOLEAN--\\|SetClickedSideA true)
      (if (Variables|/Game/Dev_Louis/02_Blueprint/03_Player/BP_ThirdPersonPlayerController_Louis.BP_ThirdPersonPlayerController_Louis_C|GetIsUsingPolaroid (CallFunction|GetPlayerControllerLouis))
        (CallFunction|CheckEnemyinRoom)
        (elif (not (Variables|Default|GetHas%20Interact))
          (if (Variables|/Game/Dev_Louis/02_Blueprint/03_Player/BP_ThirdPersonPlayerController_Louis.BP_ThirdPersonPlayerController_Louis_C|GetAllowInteractionWithWorld _asbp_third_person_player_controller_louis)
            (Variables|Default|SetHas%20Interact true)
            (Variables|/Game/Dev_Louis/02_Blueprint/03_Player/BP_ThirdPersonPlayerController_Louis.BP_ThirdPersonPlayerController_Louis_C|SetAllowInteraction _asbp_third_person_player_controller_louis false)
            (CallFunction|Activate)))))))

(event Custom|Open_Door
  (bind _t_open_door (Variables|Default|GetT_Open_Door))
  ;[0.15 0.15 0.15 0.5] Ouverture de la porte
  (if (Variables|//--BOOLEAN--\\|GetAllow_Movement)
    (Components|Timeline|SetPlayRate _t_open_door 1.0)
    (Variables|//--FLOAT--\\|SetDelay (Components|Timeline|GetTimelineLength _t_open_door))
    (bind _deltatime (Timeline|T_Open_Door PlayFromStart)
      (:Update
        (Transformation|SetActorRelativeRotation (Math|Rotator|MakeRotator 0.0 0.0 (Math|Float|Lerp (Variables|//--FLOAT--\\|GetClose_Position) (Variables|//--FLOAT--\\|GetOpen_Position) _deltatime))))
      (:Finished
        (Variables|Default|SetHas%20Interact false)
        (if (Variables|//--BOOLEAN--\\|GetClickedSideA)
          (Default|CallTargetMovement (CallFunction|GetPlayerControllerLouis) (Transformation|GetActorLocation (Variables|//--TARGETPOINT--\\|GetTargetPoint_Out_B)) 0.0)
          (else
            (Default|CallTargetMovement (CallFunction|GetPlayerControllerLouis) (Transformation|GetActorLocation (Variables|//--TARGETPOINT--\\|GetTargetPoint_Out_A)) 0.0)))
        (Utilities|FlowControl|Delay (Variables|//--FLOAT--\\|GetDelay))
        (Components|Timeline|SetPlayRate (Variables|Default|GetT_Open_Door) 1.0)
        ;;[0.9156 0 0 0.5] À MODIFIER POUR UN RENDU PROPRE
        (CallFunction|ChangeRoom)
        (Transformation|SetActorTransform (CallFunction|GetPlayerCharacterLouis) (Transformation|GetActorTransform (Variables|//--TARGETPOINT--\\|GetSpawnInRoom)))
        (bind _output_get (Variables|//--BOOLEAN--\\|SetAllow_Movement false))
        (Variables|//--BOOLEAN--\\|SetClickedSideA _output_get)
        (Variables|/Game/Dev_Louis/02_Blueprint/03_Player/BP_ThirdPersonPlayerController_Louis.BP_ThirdPersonPlayerController_Louis_C|SetAllowInteraction (CallFunction|GetPlayerControllerLouis) true)
        (Variables|Default|SetPlayer_Is_In_Range false)
        (bind _deltatime_2 (Timeline|T_Close_Door Play)
          (:Update
            (Transformation|SetActorRelativeRotation (Math|Rotator|MakeRotator 0.0 0.0 (Math|Float|Lerp (Variables|//--FLOAT--\\|GetClose_Position) (Variables|//--FLOAT--\\|GetOpen_Position) _deltatime_2)))))))))

(event EventBeginPlay
  (if (Variables|Default|GetDoorToUnlock)
    (Rendering|SetVisibility (Variables|Default|GetDoor) false false)
    (Variables|Default|SetLockedDoor true)))

(event EventActivate
  ;[0.15 0.15 0.15 0.5] Activation
  (if (Variables|Default|GetHas%20Interact)
    (if (Variables|Default|GetPlayer_Is_In_Range)
      (Variables|//--BOOLEAN--\\|SetAllow_Movement true)
      (CallFunction|OpenDoor)
      (elif (Variables|//--BOOLEAN--\\|GetClickedSideA)
        ;;[0.15 0.15 0.15 0.5] Si cliqué sur la face A
        (Default|CallTargetMovement (CallFunction|GetPlayerControllerLouis) (Transformation|GetActorLocation (Variables|//--TARGETPOINT--\\|GetTargetPoint_In_A)) 0.0)
        (else
          ;;[0.15 0.15 0.15 0.5] Si cliqué sur la face B
          (Default|CallTargetMovement (CallFunction|GetPlayerControllerLouis) (Transformation|GetActorLocation (Variables|//--TARGETPOINT--\\|GetTargetPoint_In_B)) 0.0))))))

(event EventTick
  (params (DeltaSeconds :type Float%20%28single-precision%29))
  ;[0.7565 0.01015 0 0.5] Check si le joueur utilise Capacité 1 À OPTIMISER !!!!
  (if (Variables|/Game/Dev_Louis/02_Blueprint/03_Player/BP_ThirdPersonPlayerController_Louis.BP_ThirdPersonPlayerController_Louis_C|GetIsUsingPolaroid (CallFunction|GetPlayerControllerLouis))
    (CallFunction|Glow false)
    (else
      (CallFunction|Glow true))))

(fn ConstructionScript)

(fn ChangeRoom
  (Default|Moveto (CallFunction|GetPlayerControllerLouis) (Variables|Default|GetRoom)))

(fn Glow
  (params (Reverse :type Boolean))
  (if Reverse
    (Rendering|Material|SetMaterial (Variables|Default|GetDoor) 0 "/Game/Art_Dev_Common/Materials/M_Door.M_Door")
    (elif (Utilities|Array|ContainsItem (Variables|/Game/Dev_Louis/02_Blueprint/01_Game_Management/Rooms/BP_DA_Rooms.BP_DA_Rooms_C|GetNearRooms (Variables|/Game/Dev_Louis/02_Blueprint/03_Player/BP_ThirdPersonPlayerController_Louis.BP_ThirdPersonPlayerController_Louis_C|GetCurrentRoom (CallFunction|GetPlayerControllerLouis))) (Variables|Default|GetRoom))
      (Rendering|Material|SetMaterial (Variables|Default|GetDoor) 0 "/Engine/EngineDebugMaterials/BoneWeightMaterial.BoneWeightMaterial"))))

(fn CheckEnemyinRoom
  (bind _asbp_third_person_player_controller_louis (CallFunction|GetPlayerControllerLouis))
  (bind _ui (Variables|/Game/Dev_Louis/02_Blueprint/03_Player/BP_ThirdPersonPlayerController_Louis.BP_ThirdPersonPlayerController_Louis_C|GetUI _asbp_third_person_player_controller_louis))
  (Variables|/Game/Dev_Louis/02_Blueprint/03_Player/BP_ThirdPersonPlayerController_Louis.BP_ThirdPersonPlayerController_Louis_C|SetIsUsingPolaroid _asbp_third_person_player_controller_louis false)
  (bind _output_get (Variables|/Game/Dev_Louis/02_Blueprint/03_Player/BP_ThirdPersonPlayerController_Louis.BP_ThirdPersonPlayerController_Louis_C|SetCartridges _asbp_third_person_player_controller_louis (- (Variables|/Game/Dev_Louis/02_Blueprint/03_Player/BP_ThirdPersonPlayerController_Louis.BP_ThirdPersonPlayerController_Louis_C|GetCartridges _asbp_third_person_player_controller_louis) 1)))
  (Default|UpdateCartridges _ui (Utilities|Text|ToText(Integer) _output_get))
  (Widget|SetVisibility _ui "Visible")
  (if (Variables|/Game/Dev_Louis/02_Blueprint/01_Game_Management/Rooms/BP_DA_Rooms.BP_DA_Rooms_C|GetEnemyHere (Variables|Default|GetRoom))
    (Development|PrintString "ENNEMI PRÉSENT" true true "(R=1.000000,G=0.000000,B=0.045142,A=1.000000)")
    (else
      (Development|PrintString "ENNEMI ABSENT" true true "(R=1.000000,G=0.000000,B=0.045186,A=1.000000)"))))

(fn UnlockDoor
  (if (Variables|Default|GetDoorToUnlock)
    (Rendering|SetVisibility (Variables|Default|GetDoor) true false)
    (Variables|Default|SetLockedDoor false)))