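; Touchable door actor tied to a Room, used to move between rooms or check them for enemies with a polaroid.
; Touching its mesh moves the player controller to that Room, or in polaroid mode ends that mode and prints whether an enemy is there.
; Tick polls polaroid mode and swaps the mesh material to highlight doors whose Room neighbors the current one.
; The touch handler itself does no adjacency check.
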(event OnInputTouchBegin(SM)
  (params (FingerIndex :type ETouchIndex%20Enum :default "Touch1") (TouchedComponent :type Primitive%20Component%20Object%20Reference))
  (bind _asbp_third_person_player_controller_louis (CallFunction|GetPlayerControllerLouis))
  (if (Variables|/Game/Dev_Louis/02_Blueprint/03_Player/BP_ThirdPersonPlayerController_Louis.BP_ThirdPersonPlayerController_Louis_C|GetIsUsingPolaroid _asbp_third_person_player_controller_louis)
    (Variables|/Game/Dev_Louis/02_Blueprint/03_Player/BP_ThirdPersonPlayerController_Louis.BP_ThirdPersonPlayerController_Louis_C|SetIsUsingPolaroid _asbp_third_person_player_controller_louis false)
    (if (Variables|/Game/Dev_Louis/02_Blueprint/01_Game_Management/Rooms/BP_DA_Rooms.BP_DA_Rooms_C|GetEnemyHere (Variables|Default|GetRoom))
      (Development|PrintString "ENNEMI PRÉSENT" true true "(R=1.000000,G=0.000000,B=0.045142,A=1.000000)")
      (else
        (Development|PrintString "ENNEMI ABSENT" true true "(R=1.000000,G=0.000000,B=0.045186,A=1.000000)")))
    (else
      (Default|Moveto _asbp_third_person_player_controller_louis (Variables|Default|GetRoom)))))

(event EventBeginPlay)

(event Collision|EventActorBeginOverlap
  (params (OtherActor :type Actor%20Object%20Reference)))

(event EventTick
  (params (DeltaSeconds :type Float%20%28single-precision%29))
  (if (Variables|/Game/Dev_Louis/02_Blueprint/03_Player/BP_ThirdPersonPlayerController_Louis.BP_ThirdPersonPlayerController_Louis_C|GetIsUsingPolaroid (CallFunction|GetPlayerControllerLouis))
    (CallFunction|Glow false)
    (else
      (CallFunction|Glow true))))

(fn ConstructionScript)

(fn Glow
  (params (Reverse :type Boolean))
  (if Reverse
    (Rendering|Material|SetMaterial (Variables|Default|GetSM) 0 "/Engine/BasicShapes/BasicShapeMaterial.BasicShapeMaterial")
    (elif (Utilities|Array|ContainsItem (Variables|/Game/Dev_Louis/02_Blueprint/01_Game_Management/Rooms/BP_DA_Rooms.BP_DA_Rooms_C|GetNearRooms (Variables|/Game/Dev_Louis/02_Blueprint/03_Player/BP_ThirdPersonPlayerController_Louis.BP_ThirdPersonPlayerController_Louis_C|GetCurrentRoom (CallFunction|GetPlayerControllerLouis))) (Variables|Default|GetRoom))
      (Rendering|Material|SetMaterial (Variables|Default|GetSM) 0 "/Engine/EngineDebugMaterials/BoneWeightMaterial.BoneWeightMaterial"))))