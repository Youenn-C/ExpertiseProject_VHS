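; Interactable video recorder that ends the game in victory when the player uses it while holding the enchanted hammer.
; A touch on its collider passes the player controller's interaction and hammer checks, latches HasInteract, blocks further interaction and calls Activate.
; If the player is in range, Activate spawns an effect, disables world interaction and shows the victory screen after a short delay.
; Otherwise it calls TriggerMovement.
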(event OnInputTouchBegin(Collider)
  (params (FingerIndex :type ETouchIndex%20Enum :default "Touch1") (TouchedComponent :type Primitive%20Component%20Object%20Reference))
  (if (Variables|/Game/Dev_Louis/02_Blueprint/03_Player/BP_ThirdPersonPlayerController_Louis.BP_ThirdPersonPlayerController_Louis_C|GetAllowInteraction (CallFunction|GetPlayerControllerLouis))
    (if (not (Variables|Default|GetHas%20Interact))
      (if (Variables|/Game/Dev_Louis/02_Blueprint/03_Player/BP_ThirdPersonPlayerController_Louis.BP_ThirdPersonPlayerController_Louis_C|GetAllowInteractionWithWorld (CallFunction|GetPlayerControllerLouis))
        (if (Variables|/Game/Dev_Louis/02_Blueprint/03_Player/BP_ThirdPersonPlayerController_Louis.BP_ThirdPersonPlayerController_Louis_C|GetHaveEnchantHammer (CallFunction|GetPlayerControllerLouis))
          (Variables|Default|SetHas%20Interact true)
          (Variables|/Game/Dev_Louis/02_Blueprint/03_Player/BP_ThirdPersonPlayerController_Louis.BP_ThirdPersonPlayerController_Louis_C|SetAllowInteraction (CallFunction|GetPlayerControllerLouis) false)
          (CallFunction|Activate))))))

(event EventActivate
  (bind _asbp_third_person_player_controller_louis (CallFunction|GetPlayerControllerLouis))
  (if (Variables|/Game/Dev_Louis/02_Blueprint/03_Player/BP_ThirdPersonPlayerController_Louis.BP_ThirdPersonPlayerController_Louis_C|GetHaveEnchantHammer (CallFunction|GetPlayerControllerLouis))
    (if (Variables|Default|GetPlayer_Is_In_Range)
      (Niagara|SpawnSystematLocation (Variables|Default|GetSystem%20Template) (Transformation|GetActorLocation))
      (bind _output_get (Variables|/Game/Dev_Louis/02_Blueprint/03_Player/BP_ThirdPersonPlayerController_Louis.BP_ThirdPersonPlayerController_Louis_C|SetAllowInteraction _asbp_third_person_player_controller_louis false))
      (Variables|/Game/Dev_Louis/02_Blueprint/03_Player/BP_ThirdPersonPlayerController_Louis.BP_ThirdPersonPlayerController_Louis_C|SetAllowInteractionWithWorld _asbp_third_person_player_controller_louis _output_get)
      (Utilities|FlowControl|Delay 3.0)
      (bind _returnvalue (UserInterface|CreateWidget "/Game/Dev_Youenn/02_Blueprint/03_Player/WBP_Victory_Screen.WBP_Victory_Screen_C" (CallFunction|GetPlayerControllerLouis)))
      (UserInterface|Viewport|AddtoViewport _returnvalue 0)
      (else
        (CallFunction|TriggerMovement)))))

(fn ConstructionScript
  (|CallParentFunction))