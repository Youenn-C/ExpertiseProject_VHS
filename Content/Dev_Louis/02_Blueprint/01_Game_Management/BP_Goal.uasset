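; BP_Goal is an ordered objective that the player collects by touching its mesh.
; A touch unlocks its checkpoint on the Louis third-person controller only if the previous one is current, otherwise it prints that other objectives come first.
; GoalSonar resets all rooms' goal distances, seeds the goal room and its neighbours, then estimates the rest from nearest labelled neighbours in a single ordered pass, not a full breadth-first search.
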(event OnInputTouchBegin(SM)
  (params (FingerIndex :type ETouchIndex%20Enum :default "Touch1") (TouchedComponent :type Primitive%20Component%20Object%20Reference))
  (if (== (Variables|/Game/Dev_Louis/02_Blueprint/03_Player/BP_ThirdPersonPlayerController_Louis.BP_ThirdPersonPlayerController_Louis_C|GetCheckpoint (CallFunction|GetThirdPersonControllerLouis)) (- (Variables|Default|GetCheckpointToUnlock) 1))
    (Default|GetCheckpoint (CallFunction|GetThirdPersonControllerLouis) (Variables|Default|GetCheckpointToUnlock))
    (Development|PrintString "Objectif collecté")
    (else
      (Development|PrintString "Il y a d'autres objectifs avant celui-ci"))))

(event EventBeginPlay)

(event Collision|EventActorBeginOverlap
  (params (OtherActor :type Actor%20Object%20Reference)))

(event EventTick
  (params (DeltaSeconds :type Float%20%28single-precision%29)))

(fn ConstructionScript)

(fn GoalSonar
  (bind _goalroom (Variables|Default|GetGoalRoom))
  (for _array_element (Variables|/Game/Dev_Louis/02_Blueprint/03_Player/BP_ThirdPersonPlayerController_Louis.BP_ThirdPersonPlayerController_Louis_C|GetAllRooms (CallFunction|GetThirdPersonControllerLouis))
    (Variables|/Game/Dev_Louis/02_Blueprint/01_Game_Management/Rooms/BP_DA_Rooms.BP_DA_Rooms_C|SetDistanceFromGoal _array_element -1))
  (bind _output_get (LocalVariables|SetIndice 0))
  (Variables|/Game/Dev_Louis/02_Blueprint/01_Game_Management/Rooms/BP_DA_Rooms.BP_DA_Rooms_C|SetDistanceFromGoal _goalroom _output_get)
  (bind _output_get_2 (LocalVariables|SetIndice 1))
  (for _array_element_2 (Variables|/Game/Dev_Louis/02_Blueprint/01_Game_Management/Rooms/BP_DA_Rooms.BP_DA_Rooms_C|GetNearRooms _goalroom)
    (Variables|/Game/Dev_Louis/02_Blueprint/01_Game_Management/Rooms/BP_DA_Rooms.BP_DA_Rooms_C|SetDistanceFromGoal _array_element_2 _output_get_2))
  (for _array_element_3 (Variables|/Game/Dev_Louis/02_Blueprint/03_Player/BP_ThirdPersonPlayerController_Louis.BP_ThirdPersonPlayerController_Louis_C|GetAllRooms (CallFunction|GetThirdPersonControllerLouis))
    (LocalVariables|SetIndice 15)
    (if (== (Variables|/Game/Dev_Louis/02_Blueprint/01_Game_Management/Rooms/BP_DA_Rooms.BP_DA_Rooms_C|GetDistanceFromGoal _array_element_3) -1)
      (bind _array_element_4 (Utilities|Array|ForEachLoopwithBreak (Variables|/Game/Dev_Louis/02_Blueprint/01_Game_Management/Rooms/BP_DA_Rooms.BP_DA_Rooms_C|GetNearRooms _array_element_3))
        (:LoopBody
          (if (> (Variables|/Game/Dev_Louis/02_Blueprint/01_Game_Management/Rooms/BP_DA_Rooms.BP_DA_Rooms_C|GetDistanceFromGoal _array_element_4) -1)
            (if (< (Variables|/Game/Dev_Louis/02_Blueprint/01_Game_Management/Rooms/BP_DA_Rooms.BP_DA_Rooms_C|GetDistanceFromGoal _array_element_4) (LocalVariables|GetIndice))
              (LocalVariables|SetIndice (Variables|/Game/Dev_Louis/02_Blueprint/01_Game_Management/Rooms/BP_DA_Rooms.BP_DA_Rooms_C|GetDistanceFromGoal _array_element_4))
              (LocalVariables|SetRoomToIncrement _array_element_3))))
        (:Completed
          (if (!= (LocalVariables|GetRoomToIncrement) 0)
            (Variables|/Game/Dev_Louis/02_Blueprint/01_Game_Management/Rooms/BP_DA_Rooms.BP_DA_Rooms_C|SetDistanceFromGoal (LocalVariables|GetRoomToIncrement) (+ (LocalVariables|GetIndice) 1))))))))