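; BP_Lure is a touch-activated, one-shot lure that maps each room's distance from the lure's room.
; On the first touch of its SM component, it runs LureSonar and sets LureActive on the third-person controller.
; LureSonar resets every room's DistanceFromLure, seeds the lure room and its NearRooms, then makes a single pass giving unmarked rooms their nearest marked neighbour's distance plus one.
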(event OnInputTouchBegin(SM)
  (params (FingerIndex :type ETouchIndex%20Enum :default "Touch1") (TouchedComponent :type Primitive%20Component%20Object%20Reference))
  (if (not (Variables|Default|GetAlreadyActived))
    (CallFunction|LureSonar)
    (Variables|/Game/Dev_Louis/02_Blueprint/03_Player/BP_ThirdPersonPlayerController_Louis.BP_ThirdPersonPlayerController_Louis_C|SetLureActive (CallFunction|GetThirdPersonControllerLouis) true)
    (Variables|Default|SetAlreadyActived true)))

(event EventBeginPlay)

(event Collision|EventActorBeginOverlap
  (params (OtherActor :type Actor%20Object%20Reference)))

(event EventTick
  (params (DeltaSeconds :type Float%20%28single-precision%29)))

(fn ConstructionScript)

(fn LureSonar
  (bind _lureroom (Variables|Default|GetLureRoom))
  (for _array_element (Variables|/Game/Dev_Louis/02_Blueprint/03_Player/BP_ThirdPersonPlayerController_Louis.BP_ThirdPersonPlayerController_Louis_C|GetAllRooms (CallFunction|GetThirdPersonControllerLouis))
    (Variables|/Game/Dev_Louis/02_Blueprint/01_Game_Management/Rooms/BP_DA_Rooms.BP_DA_Rooms_C|SetDistanceFromLure _array_element -1))
  (bind _output_get (LocalVariables|SetIndice 0))
  (Variables|/Game/Dev_Louis/02_Blueprint/01_Game_Management/Rooms/BP_DA_Rooms.BP_DA_Rooms_C|SetDistanceFromLure _lureroom _output_get)
  (bind _output_get_2 (LocalVariables|SetIndice 1))
  (for _array_element_2 (Variables|/Game/Dev_Louis/02_Blueprint/01_Game_Management/Rooms/BP_DA_Rooms.BP_DA_Rooms_C|GetNearRooms _lureroom)
    (Variables|/Game/Dev_Louis/02_Blueprint/01_Game_Management/Rooms/BP_DA_Rooms.BP_DA_Rooms_C|SetDistanceFromLure _array_element_2 _output_get_2))
  (for _array_element_3 (Variables|/Game/Dev_Louis/02_Blueprint/03_Player/BP_ThirdPersonPlayerController_Louis.BP_ThirdPersonPlayerController_Louis_C|GetAllRooms (CallFunction|GetPlayerControllerLouis))
    (LocalVariables|SetIndice 15)
    (if (== (Variables|/Game/Dev_Louis/02_Blueprint/01_Game_Management/Rooms/BP_DA_Rooms.BP_DA_Rooms_C|GetDistanceFromLure _array_element_3) -1)
      (for _array_element_4 (Variables|/Game/Dev_Louis/02_Blueprint/01_Game_Management/Rooms/BP_DA_Rooms.BP_DA_Rooms_C|GetNearRooms _array_element_3)
        (if (> (Variables|/Game/Dev_Louis/02_Blueprint/01_Game_Management/Rooms/BP_DA_Rooms.BP_DA_Rooms_C|GetDistanceFromLure _array_element_4) -1)
          (if (< (Variables|/Game/Dev_Louis/02_Blueprint/01_Game_Management/Rooms/BP_DA_Rooms.BP_DA_Rooms_C|GetDistanceFromLure _array_element_4) (LocalVariables|GetIndice))
            (LocalVariables|SetIndice (Variables|/Game/Dev_Louis/02_Blueprint/01_Game_Management/Rooms/BP_DA_Rooms.BP_DA_Rooms_C|GetDistanceFromLure _array_element_4))
            (LocalVariables|SetRoomToIncrement _array_element_3))))
      (if (!= (LocalVariables|GetRoomToIncrement) 0)
        (Variables|/Game/Dev_Louis/02_Blueprint/01_Game_Management/Rooms/BP_DA_Rooms.BP_DA_Rooms_C|SetDistanceFromLure (LocalVariables|GetRoomToIncrement) (+ (LocalVariables|GetIndice) 1))))))