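; BP_Cartridge is a tappable cartridge pickup actor that the player collects through Louis's player controller.
; A touch on its mesh, when interaction is allowed and the player is not at maximum cartridges, calls CollectCartridge on the controller.
; It then plays a random pickup sound, destroys itself and increments the action count of the controller's Enemy, so collecting counts toward enemy actions.
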(event OnInputTouchBegin(SM)
  (params (FingerIndex :type ETouchIndex%20Enum :default "Touch1") (TouchedComponent :type Primitive%20Component%20Object%20Reference))
  (bind _asbp_third_person_player_controller_louis (CallFunction|GetPlayerControllerLouis))
  (bind _asbp_third_person_player_controller_louis_2 (CallFunction|GetPlayerControllerLouis))
  (if (Variables|/Game/Dev_Louis/02_Blueprint/03_Player/BP_ThirdPersonPlayerController_Louis.BP_ThirdPersonPlayerController_Louis_C|GetAllowInteraction _asbp_third_person_player_controller_louis_2)
    (if (not (== (Variables|/Game/Dev_Louis/02_Blueprint/03_Player/BP_ThirdPersonPlayerController_Louis.BP_ThirdPersonPlayerController_Louis_C|GetCartridges _asbp_third_person_player_controller_louis_2) (Variables|/Game/Dev_Louis/02_Blueprint/03_Player/BP_ThirdPersonPlayerController_Louis.BP_ThirdPersonPlayerController_Louis_C|GetMaxCartridges _asbp_third_person_player_controller_louis_2)))
      (Default|CollectCartridge _asbp_third_person_player_controller_louis 2)
      (Audio|PlaySound2D (.OutItem (Utilities|Array|Random (Variables|Default|GetSoundsEffects))) 1.0 1.0 0.0 0 0)
      (Actor|DestroyActor)
      (Default|IncrementActions (Variables|/Game/Dev_Louis/02_Blueprint/03_Player/BP_ThirdPersonPlayerController_Louis.BP_ThirdPersonPlayerController_Louis_C|GetEnemy _asbp_third_person_player_controller_louis) 1))))

(event EventBeginPlay)

(event Collision|EventActorBeginOverlap
  (params (OtherActor :type Actor%20Object%20Reference)))

(event EventTick
  (params (DeltaSeconds :type Float%20%28single-precision%29)))

(fn ConstructionScript)