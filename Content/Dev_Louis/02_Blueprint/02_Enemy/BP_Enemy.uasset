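; Enemy that moves between connected rooms in a graph, skipping safe zones, and prints a loss message when it lands in the player's room.
; Move picks a random neighbor in phase 0, or the neighbor with the lowest DistanceFromPlayer in phase 1, which BeginPlay sets.
; Each move updates the rooms' EnemyHere flags and prints the enemy's location.
; ShortestWay is an unfinished pathfinding search that Move does not use.
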(event EventBeginPlay
  (Variables|Default|SetPhase 1))

(fn ConstructionScript)

(fn Move
  (Variables|/Game/Dev_Louis/02_Blueprint/01_Game_Management/Rooms/BP_DA_Rooms.BP_DA_Rooms_C|SetEnemyHere (Variables|Default|GetCurrentRoom) false)
  (Utilities|Array|Clear (Variables|Default|GetAvailableRooms))
  (for _array_element (Variables|/Game/Dev_Louis/02_Blueprint/01_Game_Management/Rooms/BP_DA_Rooms.BP_DA_Rooms_C|GetNearRooms (Variables|Default|GetCurrentRoom))
    (if (not (Variables|/Game/Dev_Louis/02_Blueprint/01_Game_Management/Rooms/BP_DA_Rooms.BP_DA_Rooms_C|GetSafeZone _array_element))
      (Utilities|Array|Add (Variables|Default|GetAvailableRooms) _array_element)))
  (if (== (Variables|Default|GetPhase) 0)
    (bind _output_get (Variables|Default|SetCurrentRoom (.OutItem (Utilities|Array|Random (Variables|Default|GetAvailableRooms)))))
    (Variables|/Game/Dev_Louis/02_Blueprint/01_Game_Management/Rooms/BP_DA_Rooms.BP_DA_Rooms_C|SetEnemyHere _output_get true)
    (Development|PrintString (Utilities|String|Append "L'ennemi est dans : " (Variables|/Game/Dev_Louis/02_Blueprint/01_Game_Management/Rooms/BP_DA_Rooms.BP_DA_Rooms_C|GetName _output_get)))
    (if (Variables|/Game/Dev_Louis/02_Blueprint/01_Game_Management/Rooms/BP_DA_Rooms.BP_DA_Rooms_C|GetPlayerHere (Variables|Default|GetCurrentRoom))
      (Development|PrintString "PERDU"))
    (elif (== (Variables|Default|GetPhase) 1)
      (Variables|Default|SetRoomToGo (.OutItem (Utilities|Array|Random (Variables|Default|GetAvailableRooms))))
      (for _array_element_2 (Variables|Default|GetAvailableRooms)
        (if (<= (Variables|/Game/Dev_Louis/02_Blueprint/01_Game_Management/Rooms/BP_DA_Rooms.BP_DA_Rooms_C|GetDistanceFromPlayer _array_element_2) (Variables|/Game/Dev_Louis/02_Blueprint/01_Game_Management/Rooms/BP_DA_Rooms.BP_DA_Rooms_C|GetDistanceFromPlayer (Variables|Default|GetRoomToGo)))
          (Variables|Default|SetRoomToGo _array_element_2)))
      (bind _output_get_2 (Variables|Default|SetCurrentRoom (Variables|Default|GetRoomToGo)))
      (Variables|/Game/Dev_Louis/02_Blueprint/01_Game_Management/Rooms/BP_DA_Rooms.BP_DA_Rooms_C|SetEnemyHere _output_get_2 true)
      (Development|PrintString (Utilities|String|Append "L'ennemi est dans : " (Variables|/Game/Dev_Louis/02_Blueprint/01_Game_Management/Rooms/BP_DA_Rooms.BP_DA_Rooms_C|GetName _output_get_2)))
      (if (Variables|/Game/Dev_Louis/02_Blueprint/01_Game_Management/Rooms/BP_DA_Rooms.BP_DA_Rooms_C|GetPlayerHere (Variables|Default|GetCurrentRoom))
        (Development|PrintString "PERDU")))))

(fn ShortestWay
  (bind _currentroom (Variables|Default|GetCurrentRoom))
  (Utilities|Array|Clear (LocalVariables|GetCheckedRooms))
  (Utilities|Map|Clear (LocalVariables|GetTab))
  (Utilities|Array|Add (LocalVariables|GetCheckedRooms) (Variables|Default|GetCurrentRoom))
  (for _array_element (Variables|/Game/Dev_Louis/02_Blueprint/01_Game_Management/Rooms/BP_DA_Rooms.BP_DA_Rooms_C|GetNearRooms _currentroom)
    (if (Variables|/Game/Dev_Louis/02_Blueprint/01_Game_Management/Rooms/BP_DA_Rooms.BP_DA_Rooms_C|GetPlayerHere _currentroom)
      (return _array_element)
      (else
        (Utilities|Map|Add (LocalVariables|GetTab) _array_element 0))))
  ;[0.15 0.15 0.15 0.5] T'es rendu là, tu checkes les near rooms des near rooms directes (pas fini)
  (bind _keypin (Utilities|Map|ForEachLoop(Map) (LocalVariables|GetTab))
    (:then
      (if (not (Utilities|Array|ContainsItem (LocalVariables|GetCheckedRooms) _keypin))
        (if (Variables|/Game/Dev_Louis/02_Blueprint/01_Game_Management/Rooms/BP_DA_Rooms.BP_DA_Rooms_C|GetPlayerHere _keypin)
          _)))))