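; Blueprint function library of shared getters for the game's common framework classes.
; Getters cast player index 0's controller or pawn to the Youenn and Louis controller and character classes, and the game instance to BP_VHS_Instance.
; ReloadSavable is the exception: it finds every BP_Savable_Objects actor in the world and calls LoadSavable on each.
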(fn GetPlayerControllerYouenn
  (bind _asbp_player_controller_youenn (Utilities|Casting|CastToBP_Player_Controller_Youenn (Game|GetPlayerController 0)))
  (return _asbp_player_controller_youenn))

(fn GetPlayerCharacterYouenn
  (bind _asbp_player_character_youenn (Utilities|Casting|CastToBP_Player_Character_Youenn (Game|Player|GetPlayerPawn 0)))
  (return _asbp_player_character_youenn))

(fn GetPlayerControllerLouis
  (bind _asbp_third_person_player_controller_louis (Utilities|Casting|CastToBP_ThirdPersonPlayerController_Louis (Game|GetPlayerController 0)))
  (return _asbp_third_person_player_controller_louis))

(fn GetVHSInstance
  (bind _asbp_vhs_instance (Utilities|Casting|CastToBP_VHS_Instance (Game|GetGameInstance)))
  (return _asbp_vhs_instance))

(fn ReloadSavable
  (bind _outactors (Actor|GetAllActorsOfClass 0 "/Game/Dev_Youenn/02_Blueprint/02_Gameplay_Elements/BP_Savable_Objects.BP_Savable_Objects_C"))
  (for _array_element _outactors
    (Default|LoadSavable _array_element)))