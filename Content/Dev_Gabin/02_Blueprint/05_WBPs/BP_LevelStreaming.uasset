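; Streams the house's room sublevels (attic, kitchen, bedrooms and others) in and out around the current room of RefLouis.
; BeginPlay loads the full level list through the recursive Loading event.
; Unload_Level targets rooms outside the current room's NearRooms, found by Différence, then chains into loading.
; Load_Level rebuilds level names from nearby rooms' display names, then requests the current room's level without making it visible.
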(event Custom|Loading
  (bind _levelloaded (Variables|Default|GetLevelLoaded))
  (bind _levelglobal (Variables|Default|GetLevelGlobal))
  ;[0.15 0.15 0.15 0.5] Load Once
  (Class|GameplayStatics|LoadStreamLevelbySoftObjectPtr (Utilities|Array|Get(acopy) _levelglobal _levelloaded) true false)
  (Math|Integer|IncrementInt (Variables|Default|GetLevelLoaded)
    (:%20%20
      (if (<= _levelloaded (Utilities|Array|Length _levelglobal))
        (CallFunction|Loading)))))

(event Custom|Load_Level
  (for _array_element (Variables|/Game/Dev_Louis/02_Blueprint/01_Game_Management/Rooms/BP_DA_Rooms.BP_DA_Rooms_C|GetNearRooms (Variables|/Game/Dev_Louis/02_Blueprint/03_Player/BP_ThirdPersonPlayerController_Louis.BP_ThirdPersonPlayerController_Louis_C|GetCurrentRoom (Variables|Default|GetRefLouis)))
    (if (Math|Boolean|ORBoolean (Utilities|Enum|Equal(Enum) (Utilities|String|Right (Utilities|GetDisplayName _array_element) 1) "1") (Utilities|Enum|Equal(Enum) (Utilities|String|Right (Utilities|GetDisplayName _array_element) 1) "2") (Utilities|Enum|Equal(Enum) (Utilities|String|Right (Utilities|GetDisplayName _array_element) 1) "3"))
      (Game|LoadStreamLevel(byName) (Utilities|String|StringToName (Utilities|String|Append "Lvl_" (Utilities|String|LeftChop (Utilities|String|RightChop (Utilities|GetDisplayName _array_element) 3) 1) "_00" (Utilities|String|Right (Utilities|GetDisplayName _array_element) 1))) true)
      (Development|PrintString (Utilities|String|Append "Lvl_" (Utilities|String|LeftChop (Utilities|String|RightChop (Utilities|GetDisplayName _array_element) 3) 1) "_00" (Utilities|String|Right (Utilities|GetDisplayName _array_element) 1)))
      (else
        (Game|LoadStreamLevel(byName) (Utilities|String|StringToName (Utilities|String|Append "Lvl_" (Utilities|String|RightChop (Utilities|GetDisplayName _array_element) 3))) true)
        (Development|PrintString (Utilities|String|Append "Lvl_" (Utilities|String|RightChop (Utilities|GetDisplayName _array_element) 3))))))
  (CallFunction|LoadNextRoom))

(event Custom|Unload_Level
  ;[0.15 0.15 0.15 0.5] Unloading
  (if (Variables|Default|GetDifferent)
    (bind _roomstounload (CallFunction|Différence)))
  (for _array_element _roomstounload
    (Game|UnloadStreamLevel(byName) (Utilities|String|StringToName (Utilities|GetDisplayName _array_element)) false)
    (Variables|Default|SetLevelUnloaded (+ (Variables|Default|GetLevelUnloaded) 1))
    (if (<= (Variables|Default|GetLevelUnloaded) (Utilities|Array|Length _roomstounload))
      (CallFunction|UnloadLevel)
      (Variables|Default|SetDifferent false)
      (else
        (CallFunction|LoadLevel)
        (Variables|Default|SetDifferent true)))
    (Development|PrintString "Hello")))

(event Custom|Load_NextRoom
  (Game|LoadStreamLevel(byName) (Utilities|String|StringToName (Utilities|GetDisplayName (Variables|/Game/Dev_Louis/02_Blueprint/03_Player/BP_ThirdPersonPlayerController_Louis.BP_ThirdPersonPlayerController_Louis_C|GetCurrentRoom (Variables|Default|GetRefLouis)))) false))

(event EventBeginPlay
  (Variables|Default|SetLevelGlobal (Utilities|Array|MakeArray "/Game/Level_Design/Lvl_Attic_001.Lvl_Attic_001" "/Game/Level_Design/Lvl_Bathroom_001.Lvl_Bathroom_001" "/Game/Level_Design/Lvl_Bathroom_002.Lvl_Bathroom_002" "/Game/Level_Design/Lvl_Bedroom_001.Lvl_Bedroom_001" "/Game/Level_Design/Lvl_Bedroom_002.Lvl_Bedroom_002" "/Game/Level_Design/Lvl_Bedroom_003.Lvl_Bedroom_003" "/Game/Level_Design/Lvl_Corridor_001.Lvl_Corridor_001" "/Game/Level_Design/Lvl_Deskroom_001.Lvl_Deskroom_001" "/Game/Level_Design/Lvl_Dinningroom_001.Lvl_Dinningroom_001" "/Game/Level_Design/Lvl_Garage_001.Lvl_Garage_001" "/Game/Level_Design/Lvl_Kitchen_001.Lvl_Kitchen_001" "/Game/Level_Design/Lvl_LittleRoom_001.Lvl_LittleRoom_001" "/Game/Level_Design/Lvl_LittleRoom_002.Lvl_LittleRoom_002" "/Game/Level_Design/Lvl_TVRoom_001.Lvl_TVRoom_001"))
  (CallFunction|Loading))

(fn ConstructionScript)

(fn Différence
  (bind _reflouis (Variables|Default|GetRefLouis))
  (bind _roomstounload (Variables|Default|GetRoomsToUnload))
  (for _array_element (Variables|/Game/Dev_Louis/02_Blueprint/03_Player/BP_ThirdPersonPlayerController_Louis.BP_ThirdPersonPlayerController_Louis_C|GetAllRooms _reflouis)
    (if (not (Utilities|Array|ContainsItem (Variables|/Game/Dev_Louis/02_Blueprint/01_Game_Management/Rooms/BP_DA_Rooms.BP_DA_Rooms_C|GetNearRooms (Variables|/Game/Dev_Louis/02_Blueprint/03_Player/BP_ThirdPersonPlayerController_Louis.BP_ThirdPersonPlayerController_Louis_C|GetCurrentRoom _reflouis)) _array_element))
      (Utilities|Array|SetArrayElem _roomstounload 0 _array_element true)))
  (return _roomstounload))