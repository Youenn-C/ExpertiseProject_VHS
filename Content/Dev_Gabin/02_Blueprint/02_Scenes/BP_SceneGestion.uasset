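; Scene manager that teleports the player between grid-named rooms (letter A–C plus number) and streams their levels.
; On BeginPlay it spawns an interactable TV, creates its layout widget and, after a load delay, caches names and locations of "Scenes"-tagged actors.
; IndexSetup marks the current room and its row/column neighbours; UpdatingAdjacentRooms recursively loads those "Lvl_" levels and unloads the rest.
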(event Custom|UpdatingAdjacentRooms
  (if (Utilities|Enum|Equal(Enum) (Utilities|Array|Get(acopy) (Variables|Default|GetScenesString) (Variables|Default|GetRoomCheck)) (Utilities|Array|Get(acopy) (Variables|Default|GetScenesAdjacent) (Variables|Default|GetRoomCheck)))
    (Game|LoadStreamLevel(byName) (Utilities|String|StringToName (Utilities|String|Append "Lvl_" (Utilities|Array|Get(acopy) (Variables|Default|GetScenesString) (Variables|Default|GetRoomCheck)))) true)
    (else
      (Game|UnloadStreamLevel(byName) (Utilities|String|StringToName (Utilities|String|Append "Lvl_" (Utilities|Array|Get(acopy) (Variables|Default|GetScenesString) (Variables|Default|GetRoomCheck)))) false)))
  (bind _output_get (Variables|Default|SetRoomCheck (+ (Variables|Default|GetRoomCheck) 1)))
  (if (< _output_get (Utilities|Array|Length (Variables|Default|GetScenesString)))
    (CallFunction|UpdatingAdjacentRooms)
    (else
      (Variables|Default|SetRoomCheck 0))))

(event Custom|ShowUI
  (UserInterface|Viewport|AddtoViewport (stale EventBeginPlay _returnvalue_2) 0))

(event EventTick
  (params (DeltaSeconds :type Float%20%28single-precision%29)))

(event EventBeginPlay
  (bind _returnvalue (Game|SpawnActorfromClass "/Game/Dev_Gabin/02_Blueprint/02_Scenes/BP_InteractableTV.BP_InteractableTV_C" (Variables|Default|GetSpawn%20Transform) "AlwaysSpawn" "MultiplyWithRoot" 0 0))
  (Variables|/Game/Dev_Gabin/02_Blueprint/02_Scenes/BP_InteractableTV.BP_InteractableTV_C|SetRef _returnvalue self)
  (bind _returnvalue_2 (UserInterface|CreateWidget "/Game/Dev_Gabin/02_Blueprint/05_WBPs/WBP_TV_Layout.WBP_TV_Layout_C"))
  (Variables|/Game/Dev_Gabin/02_Blueprint/05_WBPs/WBP_TV_Layout.WBP_TV_Layout_C|SetSceneRef _returnvalue_2 self)
  (Variables|Default|SetABCDref (Utilities|Array|MakeArray "A" "B" "C"))
  ;[0.15 0.15 0.15 0.5] Function Has to Wait For levels To load Before Being Executed
  (Utilities|FlowControl|Delay 2.0)
  (CallFunction|GetScenesandOrderThem))

(fn ConstructionScript)

(fn GetScenesandOrderThem
  ;[0.15 0.15 0.15 0.5] Get Actors -> Add Their Name To String Array
  (bind _asstatic_mesh_actor (Utilities|Casting|CastToStaticMeshActorClass "/Script/Engine.StaticMeshActor"))
  (bind _outactors (Actor|GetAllActorsOfClasswithTag _asstatic_mesh_actor "Scenes"))
  (bind _output_get (Variables|Default|SetSceneActors _outactors))
  (for (_array_element _array_index) _output_get
    (Utilities|Array|SetArrayElem (Variables|Default|GetScenesString) _array_index (Utilities|GetDisplayName _array_element) true)
    ;[0.15 0.15 0.15 0.5] Sorts The Array By Names / Numbers
    (Utilities|Array|SetArrayElem (Variables|Default|GetLocationsActors) _array_index (Transformation|GetActorLocation _array_element) true)))

(fn SetUpSpawnLocations
  (params (CurrentIndexNumber :type Integer))
  (Transformation|SetActorLocation (Game|GetPlayerCharacter 0) (+ (Utilities|Array|Get(acopy) (Variables|Default|GetLocationsActors) CurrentIndexNumber) "0.000000,0.000000,35.000000") false false))

(fn GetCurrentSceneLocation
  (params (CurrentIndexNumber :type Integer))
  (bind _scenesstring (Variables|Default|GetScenesString))
  (bind _output (Utilities|Array|Get(acopy) _scenesstring CurrentIndexNumber))
  ;[0.15 0.15 0.15 0.5] Using The Index Slot From The Pressed Button, The Game Will Split The String Of The Actor, Letter And Number, Then Sets Them To Int Variables
  (for _array_element (Utilities|String|GetCharacterArrayfromString _output)
    (Variables|Default|SetNumberIndex (Math|Conversions|ToInteger(Byte) _array_element)))
  (Variables|Default|SetLetterIndex (Utilities|Array|FindItem (Variables|Default|GetABCDref) (Utilities|String|LeftChop _output 1))))

(fn IndexSetup
  (bind _numberindex (Variables|Default|GetNumberIndex))
  (bind _scenesadjacent (Variables|Default|GetScenesAdjacent))
  (bind _scenesadjacent_2 (Variables|Default|GetScenesAdjacent))
  ;[0.15 0.15 0.15 0.5] Clears The Array That Will Be Used To Store Adjacent Rooms
  ; And Cycles Through All Possibles Rooms Of The Game
  (Utilities|Array|Clear _scenesadjacent)
  (for (_array_element _array_index) (Variables|Default|GetScenesString)
    ;[0.15 0.15 0.15 0.5] There's probably an easier way to do this
    (if (or (== _numberindex (Utilities|String|RightChop _array_element 1)) (== (Variables|Default|GetLetterIndex) (Utilities|Array|FindItem (Variables|Default|GetABCDref) (Utilities|String|LeftChop _array_element 1))))
      (if (== (+ (- (Utilities|String|RightChop _array_element 1) _numberindex) (- (Utilities|Array|FindItem (Variables|Default|GetABCDref) (Utilities|String|LeftChop _array_element 1)) (Variables|Default|GetLetterIndex))) 0)
        (Utilities|Array|SetArrayElem _scenesadjacent_2 _array_index _array_element true :!label _label)
        (elif (or (== (+ (- (Utilities|String|RightChop _array_element 1) _numberindex) (- (Utilities|Array|FindItem (Variables|Default|GetABCDref) (Utilities|String|LeftChop _array_element 1)) (Variables|Default|GetLetterIndex))) 1) (== (+ (- (Utilities|String|RightChop _array_element 1) _numberindex) (- (Utilities|Array|FindItem (Variables|Default|GetABCDref) (Utilities|String|LeftChop _array_element 1)) (Variables|Default|GetLetterIndex))) -1))
          (goto _label)
          (else
            (Utilities|Array|SetArrayElem _scenesadjacent_2 _array_index "Null" true :!label _label_2))))
      (else
        (goto _label_2))))
  (return _scenesadjacent))